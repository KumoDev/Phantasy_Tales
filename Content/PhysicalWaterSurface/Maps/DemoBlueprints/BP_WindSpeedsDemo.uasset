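; Demo director Blueprint that plays a timed showcase of the water surface under different wind speed and fetch length combinations.
; On BeginPlay it goes fullscreen, adds a SceneInfo HUD and caches the camera transform.
; A delay-chained sequence then sets WaterSettings, re-runs its ConstructionEvent, updates the HUD and, after the first scene, offsets the camera from its start.
; The game quits after the last scene.
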(event `self.ReceiveBeginPlay`
  (bind _watersettings (`self.WaterSettings`))
  (bind _watersettings_2 (`self.WaterSettings`))
  (bind _watersettings_3 (`self.WaterSettings`))
  (bind _watersettings_4 (`self.WaterSettings`))
  (bind _watersettings_5 (`self.WaterSettings`))
  (bind _watersettings_6 (`self.WaterSettings`))
  (bind _watersettings_7 (`self.WaterSettings`))
  (bind _watersettings_8 (`self.WaterSettings`))
  (bind _hud_reference (`self.HUD Reference`))
  (bind _hud_reference_2 (`self.HUD Reference`))
  (bind (_initialcameratransform_location _initialcameratransform_rotation) (`KismetMathLibrary.BreakTransform` (`self.InitialCameraTransform`)))
  (bind _hud_reference_3 (`self.HUD Reference`))
  (bind (_initialcameratransform_location_2 _initialcameratransform_rotation_2) (`KismetMathLibrary.BreakTransform` (`self.InitialCameraTransform`)))
  (bind _hud_reference_4 (`self.HUD Reference`))
  (bind (_initialcameratransform_location_3 _initialcameratransform_rotation_3) (`KismetMathLibrary.BreakTransform` (`self.InitialCameraTransform`)))
  (bind _hud_reference_5 (`self.HUD Reference`))
  (bind (_initialcameratransform_location_4 _initialcameratransform_rotation_4) (`KismetMathLibrary.BreakTransform` (`self.InitialCameraTransform`)))
  (bind _hud_reference_6 (`self.HUD Reference`))
  (bind (_initialcameratransform_location_5 _initialcameratransform_rotation_5) (`KismetMathLibrary.BreakTransform` (`self.InitialCameraTransform`)))
  (bind _hud_reference_7 (`self.HUD Reference`))
  (bind (_initialcameratransform_location_6 _initialcameratransform_rotation_6) (`KismetMathLibrary.BreakTransform` (`self.InitialCameraTransform`)))
  (bind _hud_reference_8 (`self.HUD Reference`))
  (bind (_initialcameratransform_location_7 _initialcameratransform_rotation_7) (`KismetMathLibrary.BreakTransform` (`self.InitialCameraTransform`)))
  (`|ExecutionSequence`
    (:`then_0`
      ;[1 1 1] console commands
      (`KismetSystemLibrary.ExecuteConsoleCommand` "fullscreen"))
    (:`then_1`
      ;[1 1 1] HUD
      (bind _returnvalue (`|CreateWidget` "/Game/PhysicalWaterSurface/Blueprints/UI/SceneInfo.SceneInfo_C"))
      (bind _output_get (set `self.HUD Reference` _returnvalue))
      (`UserWidget.AddToViewport` _output_get 0))
    (:`then_2`
      ;[1 1 1] save initial camera transform
      (set `self.InitialCameraTransform` (`self.GetTransform` (`self.CaneraActor`))))
    (:`then_3`
      ;[1 1 1] 10 50
      (bind _output_get_2 (set `/Game/PhysicalWaterSurface/Blueprints/WaterSettings.WindSpeed` "NewEnumerator4" _watersettings_2))
      (set `/Game/PhysicalWaterSurface/Blueprints/UI/SceneInfo.WindSpeed` (`|GetEnumeratorNameAsString` _output_get_2) _hud_reference)
      (bind _output_get_3 (set `/Game/PhysicalWaterSurface/Blueprints/WaterSettings.FetchLength` "NewEnumerator0" _watersettings_2))
      (set `/Game/PhysicalWaterSurface/Blueprints/UI/SceneInfo.FetchLength` (`|GetEnumeratorNameAsString` _output_get_3) _hud_reference)
      (`/Game/PhysicalWaterSurface/Blueprints/UI/SceneInfo.UpdateHUD` _hud_reference)
      (`/Game/PhysicalWaterSurface/Blueprints/WaterSettings.ConstructionEvent` _watersettings_2)
      (`KismetSystemLibrary.Delay` (`self.SceneDelay`))
      ;[1 1 1] 20 50
      (bind _output_get_4 (set `/Game/PhysicalWaterSurface/Blueprints/WaterSettings.WindSpeed` "NewEnumerator6" _watersettings))
      (set `/Game/PhysicalWaterSurface/Blueprints/UI/SceneInfo.WindSpeed` (`|GetEnumeratorNameAsString` _output_get_4) _hud_reference_6)
      (bind _output_get_5 (set `/Game/PhysicalWaterSurface/Blueprints/WaterSettings.FetchLength` "NewEnumerator0" _watersettings))
      (set `/Game/PhysicalWaterSurface/Blueprints/UI/SceneInfo.FetchLength` (`|GetEnumeratorNameAsString` _output_get_5) _hud_reference_6)
      (`/Game/PhysicalWaterSurface/Blueprints/UI/SceneInfo.UpdateHUD` _hud_reference_6)
      (`/Game/PhysicalWaterSurface/Blueprints/WaterSettings.ConstructionEvent` _watersettings)
      (`self.K2_SetActorTransform` (`self.CaneraActor`) (`KismetMathLibrary.MakeTransform` (+ _initialcameratransform_location_5 (20.0 10.0 15.0)) (`KismetMathLibrary.ComposeRotators` _initialcameratransform_rotation_5) (0.0 0.0 0.0)) false false)
      (`KismetSystemLibrary.Delay` (`self.SceneDelay`))
      ;[1 1 1] 5 1500
      (bind _output_get_6 (set `/Game/PhysicalWaterSurface/Blueprints/WaterSettings.WindSpeed` "NewEnumerator2" _watersettings_3))
      (set `/Game/PhysicalWaterSurface/Blueprints/UI/SceneInfo.WindSpeed` (`|GetEnumeratorNameAsString` _output_get_6) _hud_reference_3)
      (bind _output_get_7 (set `/Game/PhysicalWaterSurface/Blueprints/WaterSettings.FetchLength` "NewEnumerator6" _watersettings_3))
      (set `/Game/PhysicalWaterSurface/Blueprints/UI/SceneInfo.FetchLength` (`|GetEnumeratorNameAsString` _output_get_7) _hud_reference_3)
      (`/Game/PhysicalWaterSurface/Blueprints/UI/SceneInfo.UpdateHUD` _hud_reference_3)
      (`/Game/PhysicalWaterSurface/Blueprints/WaterSettings.ConstructionEvent` _watersettings_3)
      (`self.K2_SetActorTransform` (`self.CaneraActor`) (`KismetMathLibrary.MakeTransform` (+ _initialcameratransform_location_2 (60.0 30.0 90.0)) (`KismetMathLibrary.ComposeRotators` _initialcameratransform_rotation_2) (0.0 0.0 0.0)) false false)
      (`KismetSystemLibrary.Delay` (* (`self.SceneDelay`) 1.5))
      ;[1 1 1] 10 500
      (bind _output_get_8 (set `/Game/PhysicalWaterSurface/Blueprints/WaterSettings.WindSpeed` "NewEnumerator4" _watersettings_4))
      (set `/Game/PhysicalWaterSurface/Blueprints/UI/SceneInfo.WindSpeed` (`|GetEnumeratorNameAsString` _output_get_8) _hud_reference_4)
      (bind _output_get_9 (set `/Game/PhysicalWaterSurface/Blueprints/WaterSettings.FetchLength` "NewEnumerator3" _watersettings_4))
      (set `/Game/PhysicalWaterSurface/Blueprints/UI/SceneInfo.FetchLength` (`|GetEnumeratorNameAsString` _output_get_9) _hud_reference_4)
      (`/Game/PhysicalWaterSurface/Blueprints/UI/SceneInfo.UpdateHUD` _hud_reference_4)
      (`/Game/PhysicalWaterSurface/Blueprints/WaterSettings.ConstructionEvent` _watersettings_4)
      (`self.K2_SetActorTransform` (`self.CaneraActor`) (`KismetMathLibrary.MakeTransform` (+ _initialcameratransform_location_3 (300.0 150.0 250.0)) (`KismetMathLibrary.ComposeRotators` _initialcameratransform_rotation_3) (0.0 0.0 0.0)) false false)
      (`KismetSystemLibrary.Delay` (`self.SceneDelay`))
      ;[1 1 1] 15 1500
      (bind _output_get_10 (set `/Game/PhysicalWaterSurface/Blueprints/WaterSettings.WindSpeed` "NewEnumerator5" _watersettings_5))
      (set `/Game/PhysicalWaterSurface/Blueprints/UI/SceneInfo.WindSpeed` (`|GetEnumeratorNameAsString` _output_get_10) _hud_reference_5)
      (bind _output_get_11 (set `/Game/PhysicalWaterSurface/Blueprints/WaterSettings.FetchLength` "NewEnumerator6" _watersettings_5))
      (set `/Game/PhysicalWaterSurface/Blueprints/UI/SceneInfo.FetchLength` (`|GetEnumeratorNameAsString` _output_get_11) _hud_reference_5)
      (`/Game/PhysicalWaterSurface/Blueprints/UI/SceneInfo.UpdateHUD` _hud_reference_5)
      (`/Game/PhysicalWaterSurface/Blueprints/WaterSettings.ConstructionEvent` _watersettings_5)
      (`self.K2_SetActorTransform` (`self.CaneraActor`) (`KismetMathLibrary.MakeTransform` (+ _initialcameratransform_location_4 (1300.0 500.0 800.0)) (`KismetMathLibrary.ComposeRotators` _initialcameratransform_rotation_4) (0.0 0.0 0.0)) false false)
      (`KismetSystemLibrary.Delay` (* (`self.SceneDelay`) 2.0))
      ;[1 1 1] 20 750
      (bind _output_get_12 (set `/Game/PhysicalWaterSurface/Blueprints/WaterSettings.WindSpeed` "NewEnumerator6" _watersettings_6))
      (set `/Game/PhysicalWaterSurface/Blueprints/UI/SceneInfo.WindSpeed` (`|GetEnumeratorNameAsString` _output_get_12) _hud_reference_7)
      (bind _output_get_13 (set `/Game/PhysicalWaterSurface/Blueprints/WaterSettings.FetchLength` "NewEnumerator4" _watersettings_6))
      (set `/Game/PhysicalWaterSurface/Blueprints/UI/SceneInfo.FetchLength` (`|GetEnumeratorNameAsString` _output_get_13) _hud_reference_7)
      (`/Game/PhysicalWaterSurface/Blueprints/UI/SceneInfo.UpdateHUD` _hud_reference_7)
      (`/Game/PhysicalWaterSurface/Blueprints/WaterSettings.ConstructionEvent` _watersettings_6)
      (`self.K2_SetActorTransform` (`self.CaneraActor`) (`KismetMathLibrary.MakeTransform` (+ _initialcameratransform_location_6 (800.0 300.0 800.0)) (`KismetMathLibrary.ComposeRotators` _initialcameratransform_rotation_6) (0.0 0.0 0.0)) false false)
      (`KismetSystemLibrary.Delay` (* (`self.SceneDelay`) 1.5))
      ;[1 1 1] 20 1500
      (bind _output_get_14 (set `/Game/PhysicalWaterSurface/Blueprints/WaterSettings.WindSpeed` "NewEnumerator6" _watersettings_7))
      (set `/Game/PhysicalWaterSurface/Blueprints/UI/SceneInfo.WindSpeed` (`|GetEnumeratorNameAsString` _output_get_14) _hud_reference_8)
      (bind _output_get_15 (set `/Game/PhysicalWaterSurface/Blueprints/WaterSettings.FetchLength` "NewEnumerator6" _watersettings_7))
      (set `/Game/PhysicalWaterSurface/Blueprints/UI/SceneInfo.FetchLength` (`|GetEnumeratorNameAsString` _output_get_15) _hud_reference_8)
      (`/Game/PhysicalWaterSurface/Blueprints/UI/SceneInfo.UpdateHUD` _hud_reference_8)
      (`/Game/PhysicalWaterSurface/Blueprints/WaterSettings.ConstructionEvent` _watersettings_7)
      (`self.K2_SetActorTransform` (`self.CaneraActor`) (`KismetMathLibrary.MakeTransform` (+ _initialcameratransform_location_7 (800.0 200.0 1200.0)) (`KismetMathLibrary.ComposeRotators` _initialcameratransform_rotation_7) (0.0 0.0 0.0)) false false)
      (`KismetSystemLibrary.Delay` (* (`self.SceneDelay`) 1.5))
      ;[1 1 1] 25 500
      (bind _output_get_16 (set `/Game/PhysicalWaterSurface/Blueprints/WaterSettings.WindSpeed` "NewEnumerator7" _watersettings_8))
      (set `/Game/PhysicalWaterSurface/Blueprints/UI/SceneInfo.WindSpeed` (`|GetEnumeratorNameAsString` _output_get_16) _hud_reference_2)
      (bind _output_get_17 (set `/Game/PhysicalWaterSurface/Blueprints/WaterSettings.FetchLength` "NewEnumerator3" _watersettings_8))
      (set `/Game/PhysicalWaterSurface/Blueprints/UI/SceneInfo.FetchLength` (`|GetEnumeratorNameAsString` _output_get_17) _hud_reference_2)
      (`/Game/PhysicalWaterSurface/Blueprints/UI/SceneInfo.UpdateHUD` _hud_reference_2)
      (`/Game/PhysicalWaterSurface/Blueprints/WaterSettings.ConstructionEvent` _watersettings_8)
      (`self.K2_SetActorTransform` (`self.CaneraActor`) (`KismetMathLibrary.MakeTransform` (+ _initialcameratransform_location (1000.0 300.0 800.0)) (`KismetMathLibrary.ComposeRotators` _initialcameratransform_rotation) (0.0 0.0 0.0)) false false)
      (`KismetSystemLibrary.Delay` (* (`self.SceneDelay`) 1.5))
      (`KismetSystemLibrary.QuitGame` null "Quit"))))

(event `self.ReceiveActorBeginOverlap`
  (params (OtherActor :type "Actor Object Reference")))

(event `self.ReceiveTick`
  (params (DeltaSeconds :type "Float (single-precision)")))

(fn `UserConstructionScript`)