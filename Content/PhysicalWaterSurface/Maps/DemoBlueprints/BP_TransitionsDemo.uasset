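; Demo actor for the Physical Water Surface maps that showcases timed sea state transitions, then quits the game.
; BeginPlay steps through a scripted sequence of wind speed and fetch length changes on WaterSettings, each blended over time and held with delays before the next.
; Tick writes the current wind speed and fetch length to a text render on CameraBoat.
; Some console command calls are left unconnected.
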(event `self.ReceiveBeginPlay`
  (`KismetSystemLibrary.Delay` 5.0)
  ;[1 1 1] 10 50
  (`/Game/PhysicalWaterSurface/Blueprints/WaterSettings.ChangeSeaState` (`self.WaterSettings`) (enumliteral `/Game/PhysicalWaterSurface/Blueprints/Enumerations/WindSpeeds` "NewEnumerator4") (enumliteral `/Game/PhysicalWaterSurface/Blueprints/Enumerations/FetchLengths` "NewEnumerator0") 10.0)
  (`KismetSystemLibrary.Delay` (+ 10.0 10.0))
  ;[1 1 1] 2 50
  (`/Game/PhysicalWaterSurface/Blueprints/WaterSettings.ChangeSeaState` (`self.WaterSettings`) (enumliteral `/Game/PhysicalWaterSurface/Blueprints/Enumerations/WindSpeeds` "NewEnumerator10") (enumliteral `/Game/PhysicalWaterSurface/Blueprints/Enumerations/FetchLengths` "NewEnumerator0") 10.0)
  (`KismetSystemLibrary.Delay` (+ 10.0 10.0))
  ;[1 1 1] 5 500
  (`/Game/PhysicalWaterSurface/Blueprints/WaterSettings.ChangeSeaState` (`self.WaterSettings`) (enumliteral `/Game/PhysicalWaterSurface/Blueprints/Enumerations/WindSpeeds` "NewEnumerator2") (enumliteral `/Game/PhysicalWaterSurface/Blueprints/Enumerations/FetchLengths` "NewEnumerator3") 10.0)
  (`KismetSystemLibrary.Delay` (+ 10.0 10.0))
  ;[1 1 1] 10 750
  (`/Game/PhysicalWaterSurface/Blueprints/WaterSettings.ChangeSeaState` (`self.WaterSettings`) (enumliteral `/Game/PhysicalWaterSurface/Blueprints/Enumerations/WindSpeeds` "NewEnumerator4") (enumliteral `/Game/PhysicalWaterSurface/Blueprints/Enumerations/FetchLengths` "NewEnumerator4") 10.0)
  (`KismetSystemLibrary.Delay` (+ 10.0 10.0))
  (`KismetSystemLibrary.QuitGame` null "Quit"))

(event `self.ReceiveTick`
  (params (DeltaSeconds :type "Float (single-precision)"))
  ;[1 1 1] update text
  (`TextRenderComponent.K2_SetText` (`/Game/PhysicalWaterSurface/Blueprints/CameraBoat.TextRender` (`self.CameraBoat`)) (`KismetTextLibrary.Conv_StringToText` (`KismetStringLibrary.Concat_StrStr` "Wind Speed: " (`KismetTextLibrary.Conv_TextToString` (`KismetTextLibrary.Conv_DoubleToText` (`/Game/PhysicalWaterSurface/Blueprints/WaterSettings.WindSpeedCurrent` (`self.WaterSettings`)) "HalfToEven" false 1 324 1 1)) " m/s \n" "Fetch Length: " (`KismetTextLibrary.Conv_TextToString` (`KismetTextLibrary.Conv_DoubleToText` (`/Game/PhysicalWaterSurface/Blueprints/WaterSettings.FetchLengthCurrent` (`self.WaterSettings`)) "HalfToEven" false 1 324 1 1)) " km"))))

(fn `UserConstructionScript`)