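; Buildable campfire that heals the player at first, then drains health.
; Tick sets log and rock materials from build flags and, unless both wood and stone flags are true, marks it built and writes its location to the PlayerPos parameter collection.
; When built, overlap starts looping CampfireRegen on CH_MyCharacter, switching to CampfireHealthLoss after a delay.
; Leaving clears regen immediately and health loss after a short delay.
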(event `self.ReceiveBeginPlay`)

(event `self.ReceiveTick`
  (params (DeltaSeconds :type "Float (single-precision)"))
  (`|ExecutionSequence`
    (:`then_0`
      ;[1 0 0] Cannot be built
      (if (`self.CannotBeBuilt`)
        (`PrimitiveComponent.SetMaterial` (`self.Campfire_logs`) 0 "/Game/StylizedPlains/Materials/Instances/MI_Rock.MI_Rock")
        (`PrimitiveComponent.SetMaterial` (`self.Campfire_Rocks`) 0 "/Game/redisng/trees/SpruceBark.SpruceBark")))
    (:`then_1`
      ;[0.01276 0.3512 1] To be built materials
      (if (`self.Built_Wood`)
        (`PrimitiveComponent.SetMaterial` (`self.Campfire_logs`) 0 "/Game/StylizedPlains/Materials/Instances/MI_Rock.MI_Rock")))
    (:`then_2`
      (if (`self.Build_Stone`)
        (`PrimitiveComponent.SetMaterial` (`self.Campfire_Rocks`) 0 "/Game/redisng/trees/SpruceBark.SpruceBark")))
    (:`then_3`
      ;[1 0 0.8064] Built position
      (if (not (and (`self.Built_Wood`) (`self.Build_Stone`)))
        (set `self.Campfire_Built` true)
        (`KismetMaterialLibrary.SetVectorParameterValue` "/Game/StylizedPlains/Materials/PlayerPos.PlayerPos" "CampfireLocation" (`KismetMathLibrary.Conv_VectorToLinearColor` (`SceneComponent.K2_GetComponentLocation` (`self.DefaultSceneRoot`))))))))

(event `self.Fire_Overlap.OnComponentBeginOverlap`
  (params (OverlappedComponent :type "PrimitiveComponent Object Reference") (OtherActor :type "Actor Object Reference") (OtherComp :type "PrimitiveComponent Object Reference") (OtherBodyIndex :type Integer) (bFromSweep :type Boolean) (SweepResult :type "HitResult Structure (by ref)"))
  (if (`self.Campfire_Built`)
    (bind _asch_my_character (cast `/Game/Blueprints/Character/CH_MyCharacter` OtherActor))
    (bind _returnvalue (`KismetSystemLibrary.K2_SetTimer` _asch_my_character "CampfireRegen" 0.25 true))
    (set `self.CampfireRegen_Handle` _returnvalue)
    (`KismetSystemLibrary.Delay` 10.0)
    (`KismetSystemLibrary.K2_ClearAndInvalidateTimerHandle` (`self.CampfireRegen_Handle`))
    (bind _returnvalue_2 (`KismetSystemLibrary.K2_SetTimer` _asch_my_character "CampfireHealthLoss" 0.25 true))
    (set `self.CampfireHealthLoss_Handle` _returnvalue_2)))

(event `self.Fire_Overlap.OnComponentEndOverlap`
  (params (OverlappedComponent :type "PrimitiveComponent Object Reference") (OtherActor :type "Actor Object Reference") (OtherComp :type "PrimitiveComponent Object Reference") (OtherBodyIndex :type Integer))
  (cast `/Game/Blueprints/Character/CH_MyCharacter` OtherActor)
  (`KismetSystemLibrary.K2_ClearAndInvalidateTimerHandle` (`self.CampfireRegen_Handle`))
  (`KismetSystemLibrary.Delay` 2.0)
  (`KismetSystemLibrary.K2_ClearAndInvalidateTimerHandle` (`self.CampfireHealthLoss_Handle`)))

(fn `UserConstructionScript`)