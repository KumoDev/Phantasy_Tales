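; Character Blueprint that toggles the character's look between a glowing and a normal appearance.
; SetCHGlow assigns a shared glow material to named slots on the body Mesh and the separate Hair component.
; SetCHNormal restores the standard body material instances and hair material on those same slots.
; Both events swap materials directly by slot name, and the construction script is empty.
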(event `Set CH Glow`
  (bind _mesh (`self.Mesh`))
  (bind _hair (`self.hair`))
  (`PrimitiveComponent.SetMaterialByName` _mesh "phong4" "/Game/Adin/Materials/M_Glow_Char.M_Glow_Char")
  (`PrimitiveComponent.SetMaterialByName` _mesh "phong6" "/Game/Adin/Materials/M_Glow_Char.M_Glow_Char")
  (`PrimitiveComponent.SetMaterialByName` _mesh "phong7" "/Game/Adin/Materials/M_Glow_Char.M_Glow_Char")
  (`PrimitiveComponent.SetMaterialByName` _hair "pasted__phong7" "/Game/Adin/Materials/M_Glow_Char.M_Glow_Char")
  (`PrimitiveComponent.SetMaterialByName` _hair "pasted__pasted__phong7" "/Game/Adin/Materials/M_Glow_Char.M_Glow_Char"))

(event `Set CH Normal`
  (bind _mesh (`self.Mesh`))
  (bind _hair (`self.hair`))
  (`PrimitiveComponent.SetMaterialByName` _mesh "phong4" "/Game/Character/Guardian/phong4_Inst.phong4_Inst")
  (`PrimitiveComponent.SetMaterialByName` _mesh "phong6" "/Game/Character/Guardian/phong6_Inst.phong6_Inst")
  (`PrimitiveComponent.SetMaterialByName` _mesh "phong7" "/Game/Character/Guardian/phong7_Inst.phong7_Inst")
  (`PrimitiveComponent.SetMaterialByName` _hair "pasted__phong7" "/Game/Character/Guardian/M_Hair.M_Hair")
  (`PrimitiveComponent.SetMaterialByName` _hair "pasted__pasted__phong7" "/Game/Character/Guardian/M_Hair.M_Hair"))

(fn `UserConstructionScript`)