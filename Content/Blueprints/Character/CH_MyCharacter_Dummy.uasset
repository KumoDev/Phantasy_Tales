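; CH_MyCharacter_Dummy is a character Blueprint that swaps materials on named slots of its Mesh and Hair components.
; Every Tick, a three-step sequence applies M_Glow_Char, then twice restores the Phong instances and M_Hair.
; All three branch conditions are constant true, so the regular materials overwrite the glow within the same tick.
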(event `self.ReceiveTick`
  (params (DeltaSeconds :type "Float (single-precision)"))
  (bind _mesh (`self.Mesh`))
  (bind _hair (`self.hair`))
  (bind _mesh_2 (`self.Mesh`))
  (bind _hair_2 (`self.hair`))
  (`|ExecutionSequence`
    (:`then_0`
      (if true
        (`PrimitiveComponent.SetMaterialByName` _mesh "phong4" "/Game/Adin/Materials/M_Glow_Char.M_Glow_Char")
        (`PrimitiveComponent.SetMaterialByName` _mesh "phong6" "/Game/Adin/Materials/M_Glow_Char.M_Glow_Char")
        (`PrimitiveComponent.SetMaterialByName` _mesh "phong7" "/Game/Adin/Materials/M_Glow_Char.M_Glow_Char")
        (`PrimitiveComponent.SetMaterialByName` _hair "pasted__phong7" "/Game/Adin/Materials/M_Glow_Char.M_Glow_Char")
        (`PrimitiveComponent.SetMaterialByName` _hair "pasted__pasted__phong7" "/Game/Adin/Materials/M_Glow_Char.M_Glow_Char")))
    (:`then_1`
      (if true
        (`PrimitiveComponent.SetMaterialByName` _mesh "phong4" "/Game/Character/Guardian/phong4_Inst.phong4_Inst")
        (`PrimitiveComponent.SetMaterialByName` _mesh "phong6" "/Game/Character/Guardian/phong6_Inst.phong6_Inst")
        (`PrimitiveComponent.SetMaterialByName` _mesh "phong7" "/Game/Character/Guardian/phong7_Inst.phong7_Inst")
        (`PrimitiveComponent.SetMaterialByName` _hair "pasted__phong7" "/Game/Character/Guardian/M_Hair.M_Hair")
        (`PrimitiveComponent.SetMaterialByName` _hair "pasted__pasted__phong7" "/Game/Character/Guardian/M_Hair.M_Hair")))
    (:`then_2`
      (if true
        (`PrimitiveComponent.SetMaterialByName` _mesh_2 "phong4" "/Game/Character/Guardian/phong4_Inst.phong4_Inst")
        (`PrimitiveComponent.SetMaterialByName` _mesh_2 "phong6" "/Game/Character/Guardian/phong6_Inst.phong6_Inst")
        (`PrimitiveComponent.SetMaterialByName` _mesh_2 "phong7" "/Game/Character/Guardian/phong7_Inst.phong7_Inst")
        (`PrimitiveComponent.SetMaterialByName` _hair_2 "pasted__phong7" "/Game/Character/Guardian/M_Hair.M_Hair")
        (`PrimitiveComponent.SetMaterialByName` _hair_2 "pasted__pasted__phong7" "/Game/Character/Guardian/M_Hair.M_Hair")))))

(fn `UserConstructionScript`)