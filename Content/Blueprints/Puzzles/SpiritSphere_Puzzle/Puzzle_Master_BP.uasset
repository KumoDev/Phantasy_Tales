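; Modular pipe piece for the spirit sphere puzzle, forming a pathway that is revealed as the spirit orb character travels it.
; SpawnPath makes the construction script set meshes by PathwayChoice and rotation by axis and degree presets, then clear itself.
; BeginPlay hides non-start pieces across all instances.
; Orb overlap unhides the piece and its PathwayArray, while an end pipe instead sets Completed and destroys both.
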(event `self.ReceiveBeginPlay`
  (bind _outactors (`GameplayStatics.GetAllActorsOfClass` "Puzzle_Master_BP_C"))
  (for (_array_element _array_index) _outactors
    (if (`|EnumEquality` (`/Game/Blueprints/Puzzles/SpiritSphere_Puzzle/Puzzle_Master_BP.Pathway_Choice` (`|GetArrayItem` _outactors _array_index)) "NewEnumerator3")
      (`self.SetActorHiddenInGame` false)
      (else
        (`self.SetActorHiddenInGame` _array_element true)))))

(event `self.Box.OnComponentBeginOverlap`
  (params (OverlappedComponent :type "PrimitiveComponent Object Reference") (OtherActor :type "Actor Object Reference") (OtherComp :type "PrimitiveComponent Object Reference") (OtherBodyIndex :type Integer) (bFromSweep :type Boolean) (SweepResult :type "HitResult Structure (by ref)"))
  (bind _pathway_array (`self.Pathway_array`))
  (cast `/Game/Characters/SpiritOrb/Blueprints/Spirit_orb_character` OtherActor)
  (if (`|EnumEquality` (`self.Pathway_Choice`) "NewEnumerator4")
    (set `self.Completed` true)
    (for _array_element _pathway_array
      (`self.K2_DestroyActor` _array_element))
    (`KismetSystemLibrary.Delay` 0.05)
    (`self.K2_DestroyActor`)
    (else
      (for _array_element_2 _pathway_array
        (`self.SetActorHiddenInGame` _array_element_2 false))
      (`self.SetActorHiddenInGame` false))))

(event `self.ReceiveTick`
  (params (DeltaSeconds :type "Float (single-precision)"))
  (switch `/Game/Blueprints/Puzzles/SpiritSphere_Puzzle/Puzzle_Area_Enum` "NewEnumerator0"
    (:`NewEnumerator0`
      (if (`self.Completed`)
        _))))

(fn `Pathway Rotation`
  (returns (Rotation :type "Rotator Structure"))
  (bind _pathway_degrees (`self.Pathway_Degrees`))
  (switch `/Game/Blueprints/Puzzles/SpiritSphere_Puzzle/Puzzle_Axis` (`self.Pathway_axis`)
    (:`NewEnumerator1`
      (switch `/Game/Blueprints/Puzzles/SpiritSphere_Puzzle/Puzzle_degrees` _pathway_degrees
        (:`NewEnumerator0`
          (set `self.Rotator` (struct)))
        (:`NewEnumerator1`
          (set `self.Rotator` (struct :`Pitch` 45.0)))
        (:`NewEnumerator2`
          (set `self.Rotator` (struct :`Pitch` 90.0)))
        (:`NewEnumerator3`
          (set `self.Rotator` (struct :`Pitch` 135.0)))
        (:`NewEnumerator5`
          (set `self.Rotator` (struct :`Pitch` 180.0)))
        (:`NewEnumerator6`
          (set `self.Rotator` (struct :`Pitch` 225.0)))
        (:`NewEnumerator7`
          (set `self.Rotator` (struct :`Pitch` 270.0)))
        (:`NewEnumerator8`
          (set `self.Rotator` (struct :`Pitch` 315.0)))))
    (:`NewEnumerator0`
      (switch `/Game/Blueprints/Puzzles/SpiritSphere_Puzzle/Puzzle_degrees` _pathway_degrees
        (:`NewEnumerator0`
          (set `self.Rotator` (struct)))
        (:`NewEnumerator1`
          (set `self.Rotator` (struct :`Roll` 45.0)))
        (:`NewEnumerator2`
          (set `self.Rotator` (struct :`Roll` 90.0)))
        (:`NewEnumerator3`
          (set `self.Rotator` (struct :`Roll` 135.0)))
        (:`NewEnumerator5`
          (set `self.Rotator` (struct :`Roll` 180.0)))
        (:`NewEnumerator6`
          (set `self.Rotator` (struct :`Roll` 225.0)))
        (:`NewEnumerator7`
          (set `self.Rotator` (struct :`Roll` 270.0)))
        (:`NewEnumerator8`
          (set `self.Rotator` (struct :`Roll` 315.0)))))
    (:`NewEnumerator2`
      (switch `/Game/Blueprints/Puzzles/SpiritSphere_Puzzle/Puzzle_degrees` _pathway_degrees
        (:`NewEnumerator0`
          (set `self.Rotator` (struct)))
        (:`NewEnumerator1`
          (set `self.Rotator` (struct :`Yaw` 45.0)))
        (:`NewEnumerator2`
          (set `self.Rotator` (struct :`Yaw` 90.0)))
        (:`NewEnumerator3`
          (set `self.Rotator` (struct :`Yaw` 135.0)))
        (:`NewEnumerator5`
          (set `self.Rotator` (struct :`Yaw` 180.0)))
        (:`NewEnumerator6`
          (set `self.Rotator` (struct :`Yaw` 225.0)))
        (:`NewEnumerator7`
          (set `self.Rotator` (struct :`Yaw` 270.0)))
        (:`NewEnumerator8`
          (set `self.Rotator` (struct :`Yaw` 315.0)))))
    (:`NewEnumerator3`
      (switch `/Game/Blueprints/Puzzles/SpiritSphere_Puzzle/Puzzle_degrees` _pathway_degrees
        (:`NewEnumerator0`
          (set `self.Rotator` (struct)))
        (:`NewEnumerator1`
          (set `self.Rotator` (struct :`Pitch` 45.0 :`Roll` 45.0)))
        (:`NewEnumerator2`
          (set `self.Rotator` (struct :`Pitch` 90.0 :`Roll` 90.0)))
        (:`NewEnumerator3`
          (set `self.Rotator` (struct :`Pitch` 135.0 :`Roll` 135.0)))
        (:`NewEnumerator5`
          (set `self.Rotator` (struct :`Pitch` 180.0 :`Roll` 180.0)))
        (:`NewEnumerator6`
          (set `self.Rotator` (struct :`Pitch` 225.0 :`Roll` 225.0)))
        (:`NewEnumerator7`
          (set `self.Rotator` (struct :`Pitch` 270.0 :`Roll` 270.0)))
        (:`NewEnumerator8`
          (set `self.Rotator` (struct :`Pitch` 315.0 :`Roll` 315.0)))))
    (:`NewEnumerator4`
      (switch `/Game/Blueprints/Puzzles/SpiritSphere_Puzzle/Puzzle_degrees` _pathway_degrees
        (:`NewEnumerator0`
          (set `self.Rotator` (struct)))
        (:`NewEnumerator1`
          (set `self.Rotator` (struct :`Yaw` 45.0 :`Roll` 45.0)))
        (:`NewEnumerator2`
          (set `self.Rotator` (struct :`Yaw` 90.0 :`Roll` 90.0)))
        (:`NewEnumerator3`
          (set `self.Rotator` (struct :`Yaw` 135.0 :`Roll` 135.0)))
        (:`NewEnumerator5`
          (set `self.Rotator` (struct :`Yaw` 180.0 :`Roll` 180.0)))
        (:`NewEnumerator6`
          (set `self.Rotator` (struct :`Yaw` 225.0 :`Roll` 225.0)))
        (:`NewEnumerator7`
          (set `self.Rotator` (struct :`Yaw` 270.0 :`Roll` 270.0)))
        (:`NewEnumerator8`
          (set `self.Rotator` (struct :`Yaw` 315.0 :`Roll` 315.0)))))
    (:`NewEnumerator5`
      (switch `/Game/Blueprints/Puzzles/SpiritSphere_Puzzle/Puzzle_degrees` _pathway_degrees
        (:`NewEnumerator0`
          (set `self.Rotator` (struct)))
        (:`NewEnumerator1`
          (set `self.Rotator` (struct :`Pitch` 45.0 :`Yaw` 45.0)))
        (:`NewEnumerator2`
          (set `self.Rotator` (struct :`Pitch` 90.0 :`Yaw` 90.0)))
        (:`NewEnumerator3`
          (set `self.Rotator` (struct :`Pitch` 135.0 :`Yaw` 135.0)))
        (:`NewEnumerator5`
          (set `self.Rotator` (struct :`Pitch` 180.0 :`Yaw` 180.0)))
        (:`NewEnumerator6`
          (set `self.Rotator` (struct :`Pitch` 225.0 :`Yaw` 225.0)))
        (:`NewEnumerator7`
          (set `self.Rotator` (struct :`Pitch` 270.0 :`Yaw` 270.0)))
        (:`NewEnumerator8`
          (set `self.Rotator` (struct :`Pitch` 315.0 :`Yaw` 315.0))))))
  (return (`self.Rotator`)))

(fn `Pathway_Choice_Function`
  (returns (`Cross pipe` :type Boolean) (`L Pipe` :type Boolean) (`Straight Pipe` :type Boolean) (`Start Pipe` :type Boolean) (`T Pipe` :type Boolean) (`End Pipe` :type Boolean))
  (bind _pipe_pathway (`self.Pipe_pathway`))
  (bind _pipe (`self.Pipe`))
  (switch `/Game/Blueprints/Puzzles/SpiritSphere_Puzzle/Pipe_choice_Enum` (`self.Pathway_Choice`)
    (:`NewEnumerator0`
      (`StaticMeshComponent.SetStaticMesh` _pipe "/Game/Blueprints/Puzzles/SpiritSphere_Puzzle/cross_pipe_Cross_Joint.cross_pipe_Cross_Joint")
      (bind _returnvalue (`StaticMeshComponent.SetStaticMesh` _pipe_pathway "/Game/Blueprints/Puzzles/SpiritSphere_Puzzle/cross_pipe_Cross_Joint_001.cross_pipe_Cross_Joint_001"))
      (return _returnvalue (stale _returnvalue_2) (stale _returnvalue_3) (stale _returnvalue_4) (stale _returnvalue_5) (stale _returnvalue_6)))
    (:`NewEnumerator1`
      (`StaticMeshComponent.SetStaticMesh` _pipe "/Game/Blueprints/Puzzles/SpiritSphere_Puzzle/L_Pipe_Elbow_Joint_002.L_Pipe_Elbow_Joint_002")
      (bind _returnvalue_2 (`StaticMeshComponent.SetStaticMesh` _pipe_pathway "/Game/Blueprints/Puzzles/SpiritSphere_Puzzle/L_Pipe_Elbow_Joint_000.L_Pipe_Elbow_Joint_000"))
      (return _returnvalue _returnvalue_2 (stale _returnvalue_3) (stale _returnvalue_4) (stale _returnvalue_5) (stale _returnvalue_6)))
    (:`NewEnumerator2`
      (`StaticMeshComponent.SetStaticMesh` _pipe "/Game/Blueprints/Puzzles/SpiritSphere_Puzzle/Pipe_Cylinder.Pipe_Cylinder")
      (bind _returnvalue_3 (`StaticMeshComponent.SetStaticMesh` _pipe_pathway "/Game/Blueprints/Puzzles/SpiritSphere_Puzzle/Pipe_Cylinder_001.Pipe_Cylinder_001"))
      (return _returnvalue _returnvalue_2 _returnvalue_3 (stale _returnvalue_4) (stale _returnvalue_5) (stale _returnvalue_6)))
    (:`NewEnumerator3`
      (`StaticMeshComponent.SetStaticMesh` _pipe "/Game/Blueprints/Puzzles/SpiritSphere_Puzzle/Starter_pipe_Cylinder.Starter_pipe_Cylinder")
      (bind _returnvalue_4 (`StaticMeshComponent.SetStaticMesh` _pipe_pathway "/Game/Blueprints/Puzzles/SpiritSphere_Puzzle/Starter_pipe_Cylinder_001.Starter_pipe_Cylinder_001"))
      (return _returnvalue _returnvalue_2 _returnvalue_3 _returnvalue_4 (stale _returnvalue_5) (stale _returnvalue_6)))
    (:`NewEnumerator4`
      (`StaticMeshComponent.SetStaticMesh` _pipe "/Game/Blueprints/Puzzles/SpiritSphere_Puzzle/Pipe_Cylinder.Pipe_Cylinder")
      (bind _returnvalue_5 (`StaticMeshComponent.SetStaticMesh` (`self.Pipe_pathway`) "/Game/Blueprints/Puzzles/SpiritSphere_Puzzle/Starter_pipe_Cylinder_001.Starter_pipe_Cylinder_001"))
      (return _returnvalue _returnvalue_2 _returnvalue_3 _returnvalue_4 _returnvalue_5 (stale _returnvalue_6)))
    (:`NewEnumerator5`
      (bind _returnvalue_6 (`StaticMeshComponent.SetStaticMesh` _pipe "/Game/Blueprints/Puzzles/SpiritSphere_Puzzle/T_Pipe.T_Pipe")))))

(fn `UserConstructionScript`
  (`|ExecutionSequence`
    (:`then_0`
      (if (`self.Spawn_Path`)
        (bind (_cross_pipe _l_pipe _straight_pipe _start_pipe _t_pipe _end_pipe) (`self.Pathway_Choice_Function`))
        (if _cross_pipe
          (bind _rotation (`self.Pathway Rotation` :!label _label))
          (`self.K2_SetActorRotation` _rotation)
          (set `self.Spawn_Path` false)
          (elif _l_pipe
            (goto _label)
            (elif _straight_pipe
              (goto _label)
              (elif _start_pipe
                (goto _label)
                (elif _t_pipe
                  (goto _label)
                  (elif _end_pipe
                    (goto _label)))))))))))