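; Line puzzle actor that animates a series of decal lines, one after another, when the puzzle is completed.
; Overlapping its CompletionSphere registers the puzzle on CH_MyCharacter and sets that character's PuzzleActivate flag.
; The completion event gives each line's decal a dynamic material, and a timeline drives its Distance parameter while setting PuzzleCompleted.
; The timeline's Finished pin loops back through a DoN sized to the line array, chaining the lines sequentially.
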(event `PuzzleCompleted_event`
  (bind _puzzlelines_array (`self.PuzzleLines_Array`))
  ;[1 1 1] CompletedEvent
  (bind _counter (`/Engine/EditorBlueprintResources/StandardMacros.Do N` (`KismetArrayLibrary.Array_Length` _puzzlelines_array) :!label _label)
    (:`Exit`
      (bind _decal (`DecalActor.Decal` (`|GetArrayItem` _puzzlelines_array (- _counter 1))))
      (bind _returnvalue (`KismetMaterialLibrary.CreateDynamicMaterialInstance` (`DecalComponent.GetDecalMaterial` _decal) "/Game/Blueprints/Puzzles/LinePuzzle/testDecal_Inst.testDecal_Inst"))
      (`DecalComponent.SetDecalMaterial` _decal _returnvalue)
      (bind (_direction _newtrack_0) (`Timeline|Timeline_0` :!via `PlayFromStart`)
        (:`Update`
          (`MaterialInstanceDynamic.SetScalarParameterValue` _returnvalue "Distance" _newtrack_0)
          (set `self.PuzzleCompleted` true))
        (:`Finished`
          (goto _label))))))

(event `self.ReceiveTick`
  (params (DeltaSeconds :type "Float (single-precision)")))

(event `self.CompletionSphere.OnComponentBeginOverlap`
  (params (OverlappedComponent :type "PrimitiveComponent Object Reference") (OtherActor :type "Actor Object Reference") (OtherComp :type "PrimitiveComponent Object Reference") (OtherBodyIndex :type Integer) (bFromSweep :type Boolean) (SweepResult :type "HitResult Structure (by ref)"))
  (bind _asch_my_character (cast `/Game/Blueprints/Character/CH_MyCharacter` OtherActor))
  (set `/Game/Blueprints/Character/CH_MyCharacter.LinePuzzle` self _asch_my_character)
  (set `/Game/Blueprints/Character/CH_MyCharacter.PuzzleActivate` true _asch_my_character))

(fn `UserConstructionScript`)