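; PuzzleDoor is a puzzle-gated door that animates its material and then removes itself once the linked puzzle is completed.
; Tick polls the first PuzzleChoice entry and, after a configurable delay, applies a dynamic Doorwall_Inst material to the Plane.
; A timeline drives the material's Amount parameter, and its update also feeds a fixed delay that destroys the actor.
; The completion check has no one-shot guard, so the sequence can re-trigger until destruction.
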(event `self.ReceiveTick`
  (params (DeltaSeconds :type "Float (single-precision)"))
  (if (`/Game/Blueprints/Puzzles/LinePuzzle.PuzzleCompleted` (`|GetArrayItem` (`self.PuzzleChoice`)))
    (`KismetSystemLibrary.Delay` (`self.Delay Timer`))
    (bind _returnvalue (`KismetMaterialLibrary.CreateDynamicMaterialInstance` "/Game/Enviroment/PuzzleDoors/Doorwall_Inst.Doorwall_Inst"))
    (`PrimitiveComponent.SetMaterial` (`self.Plane`) 0 _returnvalue)
    (bind (_direction _newtrack_0) (`Timeline|Timeline_0` :!via `PlayFromStart`)
      (:`Update`
        (`MaterialInstanceDynamic.SetScalarParameterValue` _returnvalue "Amount" _newtrack_0)
        (`KismetSystemLibrary.Delay` 4.5)
        (`self.K2_DestroyActor`)))))

(fn `UserConstructionScript`)