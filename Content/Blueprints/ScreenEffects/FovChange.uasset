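; Trigger volume actor that changes the player's third-person camera field of view and boom arm length while CH_MyCharacter is inside its Box.
; Begin overlap plays the FOV timeline forward, and end overlap plays separate FOV and arm timelines in reverse from their end.
; Each arm-length timeline is started from its FOV timeline's Update pin, so it restarts on every FOV update.
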(event `self.Box.OnComponentBeginOverlap`
  (params (OverlappedComponent :type "PrimitiveComponent Object Reference") (OtherActor :type "Actor Object Reference") (OtherComp :type "PrimitiveComponent Object Reference") (OtherBodyIndex :type Integer) (bFromSweep :type Boolean) (SweepResult :type "HitResult Structure (by ref)"))
  (bind _asch_my_character (cast `/Game/Blueprints/Character/CH_MyCharacter` OtherActor))
  (bind (_direction _newtrack_0) (`Timeline|FOV Change` :!via `PlayFromStart`)
    (:`Update`
      (`CameraComponent.SetFieldOfView` (`/Game/Blueprints/Character/CH_MyCharacter.TPCam` _asch_my_character) _newtrack_0)
      (bind (_direction_2 _newtrack_0_2) (`Timeline|CameraArm` :!via `PlayFromStart`)
        (:`Update`
          (set `SpringArmComponent.TargetArmLength` _newtrack_0_2 (`/Game/Blueprints/Character/CH_MyCharacter.CameraBoom` _asch_my_character)))))))

(event `self.Box.OnComponentEndOverlap`
  (params (OverlappedComponent :type "PrimitiveComponent Object Reference") (OtherActor :type "Actor Object Reference") (OtherComp :type "PrimitiveComponent Object Reference") (OtherBodyIndex :type Integer))
  (bind _asch_my_character (cast `/Game/Blueprints/Character/CH_MyCharacter` OtherActor))
  (bind (_direction _newtrack_0) (`Timeline|ReverseFov` :!via `ReverseFromEnd`)
    (:`Update`
      (`CameraComponent.SetFieldOfView` (`/Game/Blueprints/Character/CH_MyCharacter.TPCam` _asch_my_character) _newtrack_0)
      (bind (_direction_2 _newtrack_0_2) (`Timeline|CameraArmReverse` :!via `ReverseFromEnd`)
        (:`Update`
          (set `SpringArmComponent.TargetArmLength` _newtrack_0_2 (`/Game/Blueprints/Character/CH_MyCharacter.CameraBoom` _asch_my_character)))))))

(fn `UserConstructionScript`)