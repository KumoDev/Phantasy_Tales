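; Base interactable plant that grows from seedling through stem to full-grown, then can be harvested into a food item.
; Planted disables interaction and uses delays to swap meshes over GrowthTime, then enables harvesting and updates the status text.
; Interaction either sends the harvested food's item info to the instigator or picks up the unripe plant if inventory has space.
; Food actors are spawned briefly just to read their item data, then destroyed.
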(event `Planted`
  (params (Instigator :type "Actor Object Reference"))
  (bind _returnvalue (/ (* (`self.GrowthTime`) 60.0) 2.0))
  (`PrimitiveComponent.SetCollisionEnabled` (`self.InteractableArea`) "NoCollision")
  (bind _output_get (set `self.HarvestInfo` "Growing"))
  (`TextRenderComponent.K2_SetText` (`self.TextRender`) _output_get)
  (`StaticMeshComponent.SetStaticMesh` (`self.InteractableMesh`) (`self.Mesh_Seedling`))
  (`KismetSystemLibrary.Delay` _returnvalue)
  (`StaticMeshComponent.SetStaticMesh` (`self.InteractableMesh`) (`self.Mesh_Stem`))
  (`KismetSystemLibrary.Delay` _returnvalue)
  (`StaticMeshComponent.SetStaticMesh` (`self.InteractableMesh`) (`self.Mesh_FullGrown`))
  (set `self.Harvestable` true)
  (`PrimitiveComponent.SetCollisionEnabled` (`self.InteractableArea`) "QueryAndPhysics")
  (`self.GetNameOfHarvestItem`)
  (bind _output_get_2 (set `self.HarvestInfo` "Ready To Harvest"))
  (`TextRenderComponent.K2_SetText` (`self.TextRender`) _output_get_2))

(event `/Game/Blueprints/Interactables/Intefaces/BPI_Interact.Interaction`
  (params (Instigator :type "/Game/Blueprints/Character/CH_MyCharacter Object Reference"))
  (if (`self.Harvestable`)
    ;[1 1 1] Add Harvest item to inventory
    (bind _returnvalue (`|SpawnActorFromClass` (`self.HarvestedInto`) (`self.GetTransform`) "Undefined" "OverrideRootScale" null null))
    (bind _asbp_base_food (cast `/Game/Blueprints/Interactables/Food/BP_BaseFood` _returnvalue))
    (message `/Game/Blueprints/Interactables/Intefaces/BPI_Interact.Pickup` Instigator (`/Game/Blueprints/Interactables/BP_BaseItem.ItemInfo` _asbp_base_food))
    (`self.K2_DestroyActor` _returnvalue)
    (`self.K2_DestroyActor` self)
    (bind _asfarm (cast `/Game/Blueprints/Interactables/Structures/Farm` (stale `Planted` Instigator)))
    (`PrimitiveComponent.SetCollisionEnabled` (`/Game/Blueprints/Interactables/BP_BaseInteractable.InteractableArea` _asfarm) "QueryAndPhysics")
    (else
      ;[1 1 1] Standard Pickup if plant isn't harvestable
      (if (`/Game/Blueprints/Character/CH_MyCharacter.HasSpaceInInventory` Instigator)
        (message `/Game/Blueprints/Interactables/Intefaces/BPI_Interact.Pickup` Instigator (`self.ItemInfo`))
        (`self.K2_DestroyActor`)))))

(fn `GetNameOfHarvestItem`
  (bind _returnvalue (`|SpawnActorFromClass` (`self.HarvestedInto`) (`self.GetTransform`) "Undefined" "OverrideRootScale" null null))
  (bind _asbp_base_food (cast `/Game/Blueprints/Interactables/Food/BP_BaseFood` _returnvalue))
  (set `self.ObjectName` (`KismetTextLibrary.Conv_TextToString` (`.ItemName_5_2A980C29418D0ABAB98F3F802948CCBA` (break `/Game/Blueprints/Interactables/Structs/FItemInfo` (`/Game/Blueprints/Interactables/BP_BaseItem.ItemInfo` _asbp_base_food)))))
  (`self.K2_DestroyActor` _returnvalue))

(fn `UserConstructionScript`
  (`parent.UserConstructionScript`))