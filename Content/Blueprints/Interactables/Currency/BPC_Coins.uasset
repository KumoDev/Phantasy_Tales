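; Coin pickup actor that adds a fixed amount of coins to the player character.
; On BeginPlay, if Simulate is set, it enables physics on InteractableMesh and applies a small upward impulse with random positive X and Y.
; When a CH_MyCharacter overlaps InteractableArea, it calls that character's CoinManagement to give the coins, then destroys itself.
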(event `self.ReceiveBeginPlay`
  (bind _interactablemesh (`self.InteractableMesh`))
  (if (`self.Simulate?`)
    (`PrimitiveComponent.SetSimulatePhysics` _interactablemesh true)
    (`PrimitiveComponent.AddImpulse` _interactablemesh (`KismetMathLibrary.MakeVector` (`KismetMathLibrary.RandomFloatInRange` 0.0 1.0) (`KismetMathLibrary.RandomFloatInRange` 0.0 1.0) 1.0) "None" false)))

(event `self.InteractableArea.OnComponentBeginOverlap`
  (params (OverlappedComponent :type "PrimitiveComponent Object Reference") (OtherActor :type "Actor Object Reference") (OtherComp :type "PrimitiveComponent Object Reference") (OtherBodyIndex :type Integer) (bFromSweep :type Boolean) (SweepResult :type "HitResult Structure (by ref)"))
  (bind _asch_my_character (cast `/Game/Blueprints/Character/CH_MyCharacter` OtherActor))
  (`/Game/Blueprints/Character/CH_MyCharacter.CoinManagement` _asch_my_character 3.0 false)
  (`self.K2_DestroyActor`))

(fn `UserConstructionScript`
  (`parent.UserConstructionScript`))