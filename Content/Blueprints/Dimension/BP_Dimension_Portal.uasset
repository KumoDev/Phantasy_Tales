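; Dimension portal actor that plays a dissolve transition centred on itself when the player enters its Box.
; The first overlap by any actor turns off Box overlap events; for the player, it also applies stored settings to DimensionPP and enables it.
; The DimensionTransition timeline feeds its curves and the portal's location into Dimension_MPC through DissolveEffect.
; An older expanding-sphere trace for Grid-tagged components remains as unconnected, deprecated logic.
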(event `self.Box.OnComponentBeginOverlap`
  (params (OverlappedComponent :type "PrimitiveComponent Object Reference") (OtherActor :type "Actor Object Reference") (OtherComp :type "PrimitiveComponent Object Reference") (OtherBodyIndex :type Integer) (bFromSweep :type Boolean) (SweepResult :type "HitResult Structure (by ref)"))
  (bind _dimension_pp (`self.Dimension_PP`))
  (set `PrimitiveComponent.bGenerateOverlapEvents` false (`self.Box`))
  (if (== OtherActor (`GameplayStatics.GetPlayerCharacter` 0))
    (set `PostProcessComponent.Settings` (`self.Post Process Settings`) _dimension_pp)
    (set `PostProcessComponent.bEnabled` true _dimension_pp)
    (bind (_direction _dissolve_boost _dissolve_exp _dissolve_fringe _dissolve_length _dissolve_texture_amount _dissolve_transition _flare) (`Timeline|Dimension Transition` :!via `PlayFromStart`)
      (:`Update`
        (`KismetMaterialLibrary.SetScalarParameterValue` "/Game/Dimension_MPC.Dimension_MPC" "Dissolve Boost" _dissolve_boost)
        (`KismetMaterialLibrary.SetScalarParameterValue` "/Game/Dimension_MPC.Dimension_MPC" "Dissolve Exp" _dissolve_exp)
        (`KismetMaterialLibrary.SetScalarParameterValue` "/Game/Dimension_MPC.Dimension_MPC" "Dissolve Fringe" _dissolve_fringe)
        (`KismetMaterialLibrary.SetScalarParameterValue` "/Game/Dimension_MPC.Dimension_MPC" "Dissolve Length" _dissolve_length)
        (`KismetMaterialLibrary.SetScalarParameterValue` "/Game/Dimension_MPC.Dimension_MPC" "Dissolve Texture Amount" _dissolve_texture_amount)
        (`KismetMaterialLibrary.SetScalarParameterValue` "/Game/Dimension_MPC.Dimension_MPC" "Dissolve Transition" _dissolve_transition)
        (`KismetMaterialLibrary.SetScalarParameterValue` "/Game/Dimension_MPC.Dimension_MPC" "Dissolve Flare" _flare)
        (`KismetMaterialLibrary.SetVectorParameterValue` "/Game/Dimension_MPC.Dimension_MPC" "Sphere Position" (`KismetMathLibrary.Conv_VectorToLinearColor` (`self.K2_GetActorLocation`)))))))

(fn `UserConstructionScript`)