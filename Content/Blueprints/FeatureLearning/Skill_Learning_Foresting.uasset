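; Learning trigger actor that teaches the player a skill on interaction; despite the Foresting name, it sets CombatLearned on CH_MyCharacter.
; Overlapping its Box by any actor shows a NewWidgetBlueprint widget and enables input on the actor; leaving removes the widget.
; Interact sets the flag, clears the widget and destroys the Box.
; Input is never disabled, and Interact does not check for overlap.
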(event `InputAction|Interact`
  (params (Key :type "Key Structure"))
  (:`Pressed`
    (bind _asch_my_character (cast `/Game/Blueprints/Character/CH_MyCharacter` (`GameplayStatics.GetPlayerCharacter` 0)))
    (set `/Game/Blueprints/Character/CH_MyCharacter.CombatLearned` true _asch_my_character)
    (bind _foundwidgets (`WidgetBlueprintLibrary.GetAllWidgetsOfClass` "/Game/Blueprints/FeatureLearning/NewWidgetBlueprint.NewWidgetBlueprint_C"))
    (`Widget.RemoveFromParent` _foundwidgets)
    (`ActorComponent.K2_DestroyComponent` (`self.Box`))))

(event `self.Box.OnComponentBeginOverlap`
  (params (OverlappedComponent :type "PrimitiveComponent Object Reference") (OtherActor :type "Actor Object Reference") (OtherComp :type "PrimitiveComponent Object Reference") (OtherBodyIndex :type Integer) (bFromSweep :type Boolean) (SweepResult :type "HitResult Structure (by ref)"))
  (bind _returnvalue (`GameplayStatics.GetPlayerController` 0))
  (bind _returnvalue_2 (`|CreateWidget` "/Game/Blueprints/FeatureLearning/NewWidgetBlueprint.NewWidgetBlueprint_C" _returnvalue))
  (`UserWidget.AddToViewport` _returnvalue_2 0)
  (`self.EnableInput` _returnvalue))

(event `self.Box.OnComponentEndOverlap`
  (params (OverlappedComponent :type "PrimitiveComponent Object Reference") (OtherActor :type "Actor Object Reference") (OtherComp :type "PrimitiveComponent Object Reference") (OtherBodyIndex :type Integer))
  (bind _foundwidgets (`WidgetBlueprintLibrary.GetAllWidgetsOfClass` "/Game/Blueprints/FeatureLearning/NewWidgetBlueprint.NewWidgetBlueprint_C"))
  (`Widget.RemoveFromParent` _foundwidgets))

(fn `UserConstructionScript`)