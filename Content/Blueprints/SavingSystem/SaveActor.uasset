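; Interactable save point that refills the player's health and magic and saves their progress, with configurable mesh and trigger radius.
; Interaction copies transform, level name, currency, inventory, player levels, water and equipped item into the GameInstance's CurrentSave, writes its slot, and reports success through ObjectName.
; BeginPlay also restores that data, except level name, onto the player, unless LoadFromEditor or NewGame is set.
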(event `/Game/Blueprints/Interactables/Intefaces/BPI_Interact.Interaction`
  (params (Instigator :type "/Game/Blueprints/Character/CH_MyCharacter Object Reference"))
  (bind _currentsave (`self.CurrentSave`))
  (bind _currentsave_2 (`self.CurrentSave`))
  (`self.RefreshPlayerStatus` Instigator)
  (`|ExecutionSequence`
    (:`then_0`
      (set `/Game/Blueprints/SavingSystem/SaveSystem.PlayerLocation` (`self.GetTransform` Instigator) _currentsave))
    (:`then_1`
      (bind _returnvalue (`GameplayStatics.GetCurrentLevelName` true))
      (set `/Game/Blueprints/SavingSystem/SaveSystem.LevelName` _returnvalue _currentsave))
    (:`then_2`
      (set `/Game/Blueprints/SavingSystem/SaveSystem.PlayerCurrency` (`/Game/Blueprints/Character/CH_MyCharacter.CurrencyCurrent` Instigator) _currentsave))
    (:`then_3`
      (set `/Game/Blueprints/SavingSystem/SaveSystem.Inventory` (`/Game/Blueprints/Character/CH_MyCharacter.Inventory` Instigator) _currentsave))
    (:`then_4`
      (set `/Game/Blueprints/SavingSystem/SaveSystem.PlayerLevels` (`/Game/Blueprints/Character/CH_MyCharacter.PlayerLevel` Instigator) _currentsave))
    (:`then_5`
      (set `/Game/Blueprints/SavingSystem/SaveSystem.WaterLevel` (`/Game/Blueprints/Character/CH_MyCharacter.WaterCurrent` Instigator) _currentsave))
    (:`then_6`
      (bind _output_get (set `/Game/Blueprints/SavingSystem/SaveSystem.EquipedItem` (`/Game/Blueprints/Character/CH_MyCharacter.PrimaryRightHandItem` Instigator) _currentsave))
      (`KismetSystemLibrary.PrintString` (`KismetStringLibrary.Concat_StrStr` (`KismetSystemLibrary.GetDisplayName` _output_get) "===========================")))
    (:`then_7`
      (bind _returnvalue_2 (`GameplayStatics.SaveGameToSlot` _currentsave_2 (`/Game/Blueprints/SavingSystem/SaveSystem.SaveSlotName` _currentsave_2)))
      (if _returnvalue_2
        (set `self.ObjectName` "Saved")
        (else
          (set `self.ObjectName` "FailedSaved"))))))

(event `self.ReceiveBeginPlay`
  (bind _currentsave (`self.CurrentSave`))
  (bind _playerpawn (`self.PlayerPawn`))
  ;[1 1 1] Load Game Variables
  (`self.InitialiseVars`)
  (if (`self.LoadFromEditor?`)
    _
    (elif (not (`/Game/Blueprints/Character/BP_GameInstance.NewGame?` (`self.GameInstance`)))
      (`|ExecutionSequence`
        (:`then_0`
          (`self.K2_SetActorTransform` _playerpawn (`/Game/Blueprints/SavingSystem/SaveSystem.PlayerLocation` _currentsave) false false))
        (:`then_1`
          (set `/Game/Blueprints/Character/CH_MyCharacter.CurrencyCurrent` (`/Game/Blueprints/SavingSystem/SaveSystem.PlayerCurrency` _currentsave) _playerpawn))
        (:`then_2`
          (set `/Game/Blueprints/Character/CH_MyCharacter.Inventory` (`/Game/Blueprints/SavingSystem/SaveSystem.Inventory` _currentsave) _playerpawn))
        (:`then_3`
          (set `/Game/Blueprints/Character/CH_MyCharacter.WaterCurrent` (`/Game/Blueprints/SavingSystem/SaveSystem.WaterLevel` _currentsave) _playerpawn))
        (:`then_4`
          (set `/Game/Blueprints/Character/CH_MyCharacter.PlayerLevel` (`/Game/Blueprints/SavingSystem/SaveSystem.PlayerLevels` _currentsave) _playerpawn))
        (:`then_5`
          (set `/Game/Blueprints/Character/CH_MyCharacter.PrimaryRightHandItem` (`/Game/Blueprints/SavingSystem/SaveSystem.EquipedItem` _currentsave) _playerpawn))))))

(fn `InitialiseVars`
  (bind _asbp_game_instance (cast `/Game/Blueprints/Character/BP_GameInstance` (`GameplayStatics.GetGameInstance`))
    (:`then`
      (set `self.GameInstance` _asbp_game_instance)
      (set `self.CurrentSave` (`/Game/Blueprints/Character/BP_GameInstance.CurrentSave` _asbp_game_instance))
      (bind _asch_my_character (cast `/Game/Blueprints/Character/CH_MyCharacter` (`GameplayStatics.GetPlayerPawn` 0))
        (:`then`
          (set `self.PlayerPawn` _asch_my_character))
        (:`CastFailed`
          _)))
    (:`CastFailed`
      _))
  (return))

(fn `RefreshPlayerStatus`
  (params (Player :type "/Game/Blueprints/Character/CH_MyCharacter Object Reference"))
  (set `/Game/Blueprints/Character/CH_MyCharacter.CurrentHealth` (`/Game/Blueprints/Character/CH_MyCharacter.MaxHealth` Player) Player)
  (set `/Game/Blueprints/Character/CH_MyCharacter.CurrentMagic` (`/Game/Blueprints/Character/CH_MyCharacter.MaxMagic` Player) Player)
  (set `/Game/Blueprints/Character/CH_MyCharacter.MaxStamina` (`/Game/Blueprints/Character/CH_MyCharacter.MaxStamina` Player) Player))

(fn `UserConstructionScript`
  (`StaticMeshComponent.SetStaticMesh` (`self.StaticMesh`) (`self.CustomMesh`))
  (`SphereComponent.SetSphereRadius` (`self.InteractableArea`) (`self.SaveRadius`) true)
  (`parent.UserConstructionScript`))