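; HouseSummon is a build site actor that reveals a hidden house when the player has enough wood and rock.
; Overlapping the Summon component with CH_MyCharacter shows a Summon widget, sets ReadyToBuild and enables input on the actor.
; Pressing Interact checks both resource amounts without deducting them, then unhides House, destroys the Cylinder and trigger, and removes the prompt.
; No end-overlap handling exists, so readiness and input persist after leaving.
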(event `self.ReceiveBeginPlay`)

(event `self.Summon.OnComponentBeginOverlap`
  (params (OverlappedComponent :type "PrimitiveComponent Object Reference") (OtherActor :type "Actor Object Reference") (OtherComp :type "PrimitiveComponent Object Reference") (OtherBodyIndex :type Integer) (bFromSweep :type Boolean) (SweepResult :type "HitResult Structure (by ref)"))
  (bind _asch_my_character (cast `/Game/Blueprints/Character/CH_MyCharacter` OtherActor))
  (bind _returnvalue (`|CreateWidget` "/Game/UI/Summon.Summon_C"))
  (`UserWidget.AddToViewport` _returnvalue 0)
  (set `/Game/Blueprints/Character/CH_MyCharacter.ReadyToBuild` true _asch_my_character)
  (`self.EnableInput` (`GameplayStatics.GetPlayerController` 0)))

(event `InputAction|Interact`
  (params (Key :type "Key Structure"))
  (:`Pressed`
    (if (`/Game/Blueprints/Character/CH_MyCharacter.ReadyToBuild` (stale `self.Summon.OnComponentBeginOverlap` _asch_my_character))
      (if (>= (`/Game/Blueprints/Character/CH_MyCharacter.WoodAmount` (stale `self.Summon.OnComponentBeginOverlap` _asch_my_character)) 20)
        (if (>= (`/Game/Blueprints/Character/CH_MyCharacter.RockAmount` (stale `self.Summon.OnComponentBeginOverlap` _asch_my_character)) 20)
          (`SceneComponent.SetHiddenInGame` (`self.House`) false false)
          (`ActorComponent.K2_DestroyComponent` (`self.Cylinder`))
          (`ActorComponent.K2_DestroyComponent` (`self.Summon`))
          (bind _foundwidgets (`WidgetBlueprintLibrary.GetAllWidgetsOfClass` "/Game/UI/Summon.Summon_C"))
          (`Widget.RemoveFromParent` _foundwidgets))))))

(fn `UserConstructionScript`)