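; Base chest actor that the player can open with the Interact input while standing inside its Box trigger.
; Box overlap with CH_MyCharacter enables input from player controller 0 on the chest, and leaving disables it.
; Pressing Interact in the initial ChestState plays the opening animation once and switches the state, so it opens only once.
; BeginPlay also runs a visibility multi-line trace whose result is unused.
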(event `self.ReceiveBeginPlay`
  (`KismetSystemLibrary.LineTraceMulti` (0.0 0.0 0.0) (0.0 0.0 0.0) "TraceTypeQuery1"))

(event `self.Box.OnComponentBeginOverlap`
  (params (OverlappedComponent :type "PrimitiveComponent Object Reference") (OtherActor :type "Actor Object Reference") (OtherComp :type "PrimitiveComponent Object Reference") (OtherBodyIndex :type Integer) (bFromSweep :type Boolean) (SweepResult :type "HitResult Structure (by ref)"))
  (cast `/Game/Blueprints/Character/CH_MyCharacter` OtherActor)
  (`self.EnableInput` (`GameplayStatics.GetPlayerController` 0)))

(event `InputAction|Interact`
  (params (Key :type "Key Structure"))
  (:`Pressed`
    (if (`|EnumEquality` (`self.Chest_State`) "NewEnumerator0")
      (`SkeletalMeshComponent.PlayAnimation` (`self.Chest`) "/Game/Blueprints/Chest/Animations/Chest_Opening_Anim.Chest_Opening_Anim" false)
      (set `self.Chest_State` "NewEnumerator1"))))

(event `self.Box.OnComponentEndOverlap`
  (params (OverlappedComponent :type "PrimitiveComponent Object Reference") (OtherActor :type "Actor Object Reference") (OtherComp :type "PrimitiveComponent Object Reference") (OtherBodyIndex :type Integer))
  (cast `/Game/Blueprints/Character/CH_MyCharacter` OtherActor)
  (`self.DisableInput` (`GameplayStatics.GetPlayerController` 0)))

(fn `UserConstructionScript`)