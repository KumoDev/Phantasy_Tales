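; BP_InteractiveRocks scatters randomly rotated and scaled rock instances onto surfaces around the actor, using the instanced component Tree.
; Random downward traces propose points, rejected if too close to stored locations in ComparitiveVectors.
; The GenerateRocks toggle fills in the construction script, retrying failed points, while RuntimeTreeBuild runs a fast looping timer until MaxTreesToSpawn.
; ClearRocks only resets its own flag, removing nothing.
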(event `self.ReceiveBeginPlay`
  (if (`self.RuntimeTreeBuild?`)
    ;[1 0 0] READ THE NOTE, SERIOUSLY
    (bind _returnvalue (`KismetSystemLibrary.K2_SetTimerDelegate` (delegate `EventRuntimeTrees`) 0.0001 true)) ; !!!NOTE!!! NEVER EVER EVER MAKE THE TIME VALUE\nLESS THAN 0.0001, THIS IS THE SWEET SPOT \nBETWEEN SPEED & PERFORMANCE, ANY LOWER\nAND YOU MAY CRASH YOUR PROJECT\n\nSets up how often a trace will be run\nduring the spawn cycle.
    (set `self.Timer` _returnvalue)))

(event `EventRuntimeTrees`
  (bind _z (.z (`self.TempSpawnVec`)))
  (if (< (`InstancedStaticMeshComponent.GetInstanceCount` (`self.Tree`)) (`self.MaxTreesToSpawn`))
    (bind _output_get (set `self.TempSpawnVec` (`self.RandomLocation(Controlled)`)))
    (bind _outhit (`KismetSystemLibrary.LineTraceSingle` :`Start` _output_get :`End` (`KismetMathLibrary.MakeVector` (.x (`self.TempSpawnVec`)) (.y (`self.TempSpawnVec`)) (+ (- _z _z) (`self.SpawnMinHeight`))) :`TraceChannel` "TraceTypeQuery1" :`DrawDebugType` "ForOneFrame")) ; Traces landscape for location information
    (set `self.TempOVCount` 0) ; Reset per-trace overlap count
    (for _index (range (`KismetArrayLibrary.Array_Length` (`self.ComparitiveVectors`)) 1)
      (bind (_bblockinghit _binitialoverlap _time _distance _location) (`GameplayStatics.BreakHitResult` _outhit))
      (`self.OverlapChecks` _index _location))
    (if (> (`self.TempOVCount`) 0)
      _
      (elif (!= _location (0.0 0.0 0.0) :`ErrorTolerance` 2.0)
        (bind _returnvalue (`KismetMathLibrary.MakeTransform` _location (`KismetMathLibrary.MakeRotator` 0.0 0.0 (`KismetMathLibrary.RandomFloatInRange` -180.0 180.0)) (* (1.0 1.0 1.0) (`KismetMathLibrary.RandomFloatInRange` (`self.MinInstanceScale`) (`self.MaxInstanceScale`)))))
        (`InstancedStaticMeshComponent.AddInstanceWorldSpace` (`self.Tree`) _returnvalue)
        (`KismetArrayLibrary.Array_Add` (`self.ComparitiveVectors`) (.location _returnvalue))))
    (else
      (`KismetSystemLibrary.K2_PauseTimerHandle` (`self.Timer`)))))

(fn `OverlapChecks`
  (params (LoopIndex :type Integer) (HitLocation :type "Vector Structure"))
  (if (not (< (`self.MinDistanceBetweenInstances`) (`KismetMathLibrary.VSize` (- (`|GetArrayItem` (`self.ComparitiveVectors`) LoopIndex) HitLocation))))
    (set `self.TempOVCount` (+ (`self.TempOVCount`) 1)))
  (return))

(fn `RandomLocation(Controlled)`
  (returns (Location :type "Vector Structure"))
  (bind _spawndistancefromcenter (`self.SpawnDistanceFromCenter`))
  (bind _spawndistancefromcenter_2 (`self.SpawnDistanceFromCenter`))
  (bind _z (.z (`self.K2_GetActorLocation`)))
  (return (`KismetMathLibrary.MakeVector` (+ (.x (`self.K2_GetActorLocation`)) (`KismetMathLibrary.RandomFloatInRange` (* _spawndistancefromcenter -1.0) _spawndistancefromcenter)) (+ (.y (`self.K2_GetActorLocation`)) (`KismetMathLibrary.RandomFloatInRange` (* _spawndistancefromcenter_2 -1.0) _spawndistancefromcenter_2)) (+ (- _z _z) (`self.SpawnMaxHeight`)))))

(fn `UserConstructionScript`
  (bind _z (.z (`self.TempSpawnVec`)))
  (if (`self.GenerateRocks`)
    (set `self.GenerateRocks` false)
    (for _ (range (+ (`self.MaxTreesToSpawn`) 1))
      (bind _output_get (set `self.TempSpawnVec` (`self.RandomLocation(Controlled)`) :!label _label))
      (bind _outhit (`KismetSystemLibrary.LineTraceSingle` _output_get (`KismetMathLibrary.MakeVector` (.x (`self.TempSpawnVec`)) (.y (`self.TempSpawnVec`)) (+ (- _z _z) (`self.SpawnMinHeight`))) "TraceTypeQuery1" true)) ; Traces landscape for location information
      (set `self.TempOVCount` 0) ; Reset per-trace overlap count
      (for _index (range (`KismetArrayLibrary.Array_Length` (`self.ComparitiveVectors`)) 1)
        (bind (_bblockinghit _binitialoverlap _time _distance _location) (`GameplayStatics.BreakHitResult` _outhit))
        (`self.OverlapChecks` _index _location))
      (if (> (`self.TempOVCount`) 0)
        (goto _label)
        (elif (!= _location (0.0 0.0 0.0) :`ErrorTolerance` 2.0)
          (bind _returnvalue (`KismetMathLibrary.MakeTransform` _location (`KismetMathLibrary.MakeRotator` 0.0 0.0 (`KismetMathLibrary.RandomFloatInRange` -180.0 180.0)) (* (1.0 1.0 1.0) (`KismetMathLibrary.RandomFloatInRange` (`self.MinInstanceScale`) (`self.MaxInstanceScale`)))))
          (`InstancedStaticMeshComponent.AddInstanceWorldSpace` (`self.Tree`) _returnvalue) ; Adds a tree at the provided location w/ the provided\nrandom yaw and controlled random uniform scale.
          (`KismetArrayLibrary.Array_Add` (`self.ComparitiveVectors`) (.location _returnvalue)) ; Stores the location of this tree spawn for comparison\nin future placement traces for overlap checking.
          (else
            (goto _label)))))
    (elif (`self.ClearRocks`)
      (set `self.ClearRocks` false))))