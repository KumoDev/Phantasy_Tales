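; Parent Blueprint for spirit sphere spline puzzles that hands player control to a spirit orb character.
; Overlapping the Sphere trigger enables input on the actor for player 0, with no check on the overlapping actor.
; Pressing T then spawns a Spirit_orb_character at the scene root, passes this actor as its SplineReference and has the player controller possess it.
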(event `self.Sphere.OnComponentBeginOverlap`
  (params (OverlappedComponent :type "PrimitiveComponent Object Reference") (OtherActor :type "Actor Object Reference") (OtherComp :type "PrimitiveComponent Object Reference") (OtherBodyIndex :type Integer) (bFromSweep :type Boolean) (SweepResult :type "HitResult Structure (by ref)"))
  ;[1 1 1] activate puzzle
  (`self.EnableInput` (`GameplayStatics.GetPlayerController` 0)))

(event `Key|T`
  (params (Key :type "Key Structure"))
  ;[1 1 1] activate puzzle
  (:`Pressed`
    (`KismetSystemLibrary.PrintString` "Hello")
    (bind _returnvalue (`|SpawnActorFromClass` "/Game/Character/SpiritOrb/Blueprints/Spirit_orb_character.Spirit_orb_character_C" (`KismetMathLibrary.MakeTransform` (`SceneComponent.K2_GetComponentLocation` (`self.DefaultSceneRoot`))) "Undefined" "OverrideRootScale" null null))
    (set `/Game/Character/SpiritOrb/Blueprints/Spirit_orb_character.Spline_reference` self _returnvalue)
    (`Controller.Possess` (`GameplayStatics.GetPlayerController` 0) _returnvalue)))

(fn `UserConstructionScript`)