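; Pushable puzzle block that lets the player character push it and switches to physics simulation when nothing is beneath it.
; Each tick, a 500-unit down trace from the actor turns physics on when it misses, then a 200-unit trace from the box mesh turns it off on a hit.
; Four side triggers set CanPush on the overlapping CH_MyCharacter; nothing here clears it.
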(event `self.ReceiveTick`
  (params (DeltaSeconds :type "Float (single-precision)"))
  (bind _returnvalue (`self.K2_GetActorLocation`))
  (bind _movingboxmesh (`self.MovingBoxMesh`))
  (bind _returnvalue_2 (`SceneComponent.K2_GetComponentLocation` _movingboxmesh))
  (`|ExecutionSequence`
    (:`then_0`
      (bind (_outhit _returnvalue_3) (`KismetSystemLibrary.LineTraceSingle` _returnvalue (+ _returnvalue (* (* (`self.GetActorUpVector`) -1) 500.0)) "TraceTypeQuery1"))
      (if (not _returnvalue_3)
        (`PrimitiveComponent.SetSimulatePhysics` (`self.MovingBoxMesh`) true)))
    (:`then_1`
      (bind (_outhit_2 _returnvalue_4) (`KismetSystemLibrary.LineTraceSingle` :`Start` _returnvalue_2 :`End` (+ _returnvalue_2 (* (* (`SceneComponent.GetUpVector` _movingboxmesh) -1) 200.0)) :`TraceChannel` "TraceTypeQuery1" :`DrawDebugType` "ForOneFrame"))
      (if _returnvalue_4
        (`PrimitiveComponent.SetSimulatePhysics` (`self.MovingBoxMesh`) false)))))

(event `self.Side1.OnComponentBeginOverlap`
  (params (OverlappedComponent :type "PrimitiveComponent Object Reference") (OtherActor :type "Actor Object Reference") (OtherComp :type "PrimitiveComponent Object Reference") (OtherBodyIndex :type Integer) (bFromSweep :type Boolean) (SweepResult :type "HitResult Structure (by ref)"))
  (bind _asch_my_character (cast `/Game/Blueprints/Character/CH_MyCharacter` OtherActor))
  (set `/Game/Blueprints/Character/CH_MyCharacter.CanPush` true _asch_my_character))

(event `self.Side2.OnComponentBeginOverlap`
  (params (OverlappedComponent :type "PrimitiveComponent Object Reference") (OtherActor :type "Actor Object Reference") (OtherComp :type "PrimitiveComponent Object Reference") (OtherBodyIndex :type Integer) (bFromSweep :type Boolean) (SweepResult :type "HitResult Structure (by ref)"))
  (bind _asch_my_character (cast `/Game/Blueprints/Character/CH_MyCharacter` OtherActor))
  (set `/Game/Blueprints/Character/CH_MyCharacter.CanPush` true _asch_my_character))

(event `self.Side 3.OnComponentBeginOverlap`
  (params (OverlappedComponent :type "PrimitiveComponent Object Reference") (OtherActor :type "Actor Object Reference") (OtherComp :type "PrimitiveComponent Object Reference") (OtherBodyIndex :type Integer) (bFromSweep :type Boolean) (SweepResult :type "HitResult Structure (by ref)"))
  (bind _asch_my_character (cast `/Game/Blueprints/Character/CH_MyCharacter` OtherActor))
  (set `/Game/Blueprints/Character/CH_MyCharacter.CanPush` true _asch_my_character))

(event `self.Side 4.OnComponentBeginOverlap`
  (params (OverlappedComponent :type "PrimitiveComponent Object Reference") (OtherActor :type "Actor Object Reference") (OtherComp :type "PrimitiveComponent Object Reference") (OtherBodyIndex :type Integer) (bFromSweep :type Boolean) (SweepResult :type "HitResult Structure (by ref)"))
  (bind _asch_my_character (cast `/Game/Blueprints/Character/CH_MyCharacter` OtherActor))
  (set `/Game/Blueprints/Character/CH_MyCharacter.CanPush` true _asch_my_character))

(fn `UserConstructionScript`)