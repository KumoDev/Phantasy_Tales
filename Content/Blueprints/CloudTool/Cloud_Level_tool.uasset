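; Editor-time cloud level tool Blueprint that lays out a grid of mesh instances along a curving path.
; The construction script walks an Arrow component forward as a cursor, turning it by curve roll, pitch and yaw increments each loop.
; At each step it sidesteps along the right vector to add a row, then returns to the saved spine location.
; Blocks go into a Hierarchical Instanced Static Mesh, and the event graph has no active logic.
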(fn `UserConstructionScript`
  (locals (LocationTest :type "Vector Structure" :default (0.0 0.0 0.0)))
  (bind _arrow (`self.Arrow`))
  (bind _arrow_2 (`self.Arrow`))
  (bind (_returnvalue_roll _returnvalue_pitch _returnvalue_yaw) (`KismetMathLibrary.BreakRotator` (`SceneComponent.K2_GetComponentRotation` _arrow_2)))
  (bind _returnvalue (`SceneComponent.K2_GetComponentLocation` _arrow))
  (bind _returnvalue_2 (+ _returnvalue (* (`SceneComponent.GetForwardVector` _arrow) (`self.BlockDistanceXfactor`))))
  (bind _returnvalue_3 (`KismetMathLibrary.MakeTransform` _returnvalue_2 (`SceneComponent.K2_GetComponentRotation` (`self.Arrow`))))
  (for _ (range (+ (`self.Loops`) 1))
    (set `local.LocationTest` _returnvalue_2)
    (`SceneComponent.K2_SetWorldLocation` (`self.Arrow`) _returnvalue_2 false false)
    (`InstancedStaticMeshComponent.AddInstanceWorldSpace` (`self.HierarchicalInstancedStaticMesh`) _returnvalue_3)
    (`SceneComponent.K2_SetWorldRotation` _arrow_2 (`KismetMathLibrary.MakeRotator` (+ _returnvalue_roll (`self.CurveRoll`)) (+ _returnvalue_pitch (`self.CurvePitch`)) (+ _returnvalue_yaw (`self.CurveYaw`))) false false)
    (for _ (range (+ (`self.Rows`) 1))
      (`SceneComponent.K2_SetWorldLocation` _arrow_2 (+ (* (`SceneComponent.GetRightVector` _arrow) (`self.BlockDistanceYfactor`)) _returnvalue) false false)
      (`InstancedStaticMeshComponent.AddInstanceWorldSpace` (`self.HierarchicalInstancedStaticMesh`) _returnvalue_3))
    (`SceneComponent.K2_SetWorldLocation` _arrow_2 (`local.LocationTest`) false false)))