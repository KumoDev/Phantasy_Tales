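; BP_TreeTop_Pine is the felled pine top that the player harvests for wood.
; On its first hit against something other than the player or tree base class, it spawns delayed smoke at four sphere points, then enables input.
; Capsule overlap tracks player proximity and reveals the button prompt; end overlap disables input but leaves the prompt visible.
; Interacting in range hides the prompt, destroys capsule and mesh, and adds random wood.
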(event `self.ReceiveTick`
  (params (DeltaSeconds :type "Float (single-precision)")))

(event `InputAction|Interact` :consume false
  (params (Key :type "Key Structure"))
  (:`Pressed`
    (if (`self.attree`)
      (bind _asch_my_character (cast `/Game/Blueprints/Character/CH_MyCharacter` (`GameplayStatics.GetPlayerCharacter` 0)))
      (`SceneComponent.SetHiddenInGame` (`/Game/Blueprints/Character/CH_MyCharacter.AButton` _asch_my_character) true false)
      (`ActorComponent.K2_DestroyComponent` (`self.Capsule`))
      (`ActorComponent.K2_DestroyComponent` (`self.StaticMesh`))
      (bind _woodamount (`/Game/Blueprints/Character/CH_MyCharacter.WoodAmount` _asch_my_character))
      (set `/Game/Blueprints/Character/CH_MyCharacter.WoodAmount` (+ _woodamount (`KismetMathLibrary.RandomInteger` 20)) _asch_my_character)
      (`KismetSystemLibrary.PrintString` (`KismetStringLibrary.Conv_IntToString` _woodamount)))))

(event `self.Capsule.OnComponentBeginOverlap`
  (params (OverlappedComponent :type "PrimitiveComponent Object Reference") (OtherActor :type "Actor Object Reference") (OtherComp :type "PrimitiveComponent Object Reference") (OtherBodyIndex :type Integer) (bFromSweep :type Boolean) (SweepResult :type "HitResult Structure (by ref)"))
  (bind _asch_my_character (cast `/Game/Blueprints/Character/CH_MyCharacter` OtherActor))
  (`SceneComponent.SetHiddenInGame` (`/Game/Blueprints/Character/CH_MyCharacter.AButton` _asch_my_character) false false)
  (set `self.attree` true))

(event `self.Capsule.OnComponentEndOverlap`
  (params (OverlappedComponent :type "PrimitiveComponent Object Reference") (OtherActor :type "Actor Object Reference") (OtherComp :type "PrimitiveComponent Object Reference") (OtherBodyIndex :type Integer))
  (bind _asch_my_character (cast `/Game/Blueprints/Character/CH_MyCharacter` OtherActor))
  (`SceneComponent.SetHiddenInGame` (`/Game/Blueprints/Character/CH_MyCharacter.AButton` _asch_my_character) false false)
  (set `self.attree` false)
  (`self.DisableInput` (`GameplayStatics.GetPlayerController` 0)))

(event `self.StaticMesh.OnComponentHit`
  (params (HitComponent :type "PrimitiveComponent Object Reference") (OtherActor :type "Actor Object Reference") (OtherComp :type "PrimitiveComponent Object Reference") (NormalImpulse :type "Vector Structure") (Hit :type "HitResult Structure (by ref)"))
  (bind _returnvalue (`GameplayStatics.GetObjectClass` OtherActor))
  (if (!= _returnvalue "/Game/Blueprints/Character/CH_MyCharacter.CH_MyCharacter_C")
    (if (!= _returnvalue "/Game/TreeCutting/Blueprints/BP_InteractiveTreesbase.BP_InteractiveTreesbase_C")
      (`/Engine/EditorBlueprintResources/StandardMacros.DoOnce` false
        (:`Completed`
          (`KismetSystemLibrary.Delay` 0.7)
          (`GameplayStatics.SpawnEmitterAtLocation` "/Game/Adin/Cartoony-Particles/Particles/PS_Smoke2.PS_Smoke2" (`SceneComponent.K2_GetComponentLocation` (`self.Sphere`)) (struct) (3.0 3.0 3.0))
          (`GameplayStatics.SpawnEmitterAtLocation` "/Game/Adin/Cartoony-Particles/Particles/PS_Smoke2.PS_Smoke2" (`SceneComponent.K2_GetComponentLocation` (`self.Sphere2`)) (struct) (3.0 3.0 3.0))
          (`GameplayStatics.SpawnEmitterAtLocation` "/Game/Adin/Cartoony-Particles/Particles/PS_Smoke2.PS_Smoke2" (`SceneComponent.K2_GetComponentLocation` (`self.Sphere3`)) (struct) (3.0 3.0 3.0))
          (`GameplayStatics.SpawnEmitterAtLocation` "/Game/Adin/Cartoony-Particles/Particles/PS_Smoke2.PS_Smoke2" (`SceneComponent.K2_GetComponentLocation` (`self.Sphere1`)) (struct) (3.0 3.0 3.0))
          (`KismetSystemLibrary.Delay` 1.0)
          (`self.EnableInput` (`GameplayStatics.GetPlayerController` 0)))))))

(fn `UserConstructionScript`)