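; BP_Storm is a cartoony storm cloud actor with cloud puffs, a lightning plane and rain flash, but none of its graph logic is wired to run.
; The disconnected LightningFlash timeline would drive lightning color parameters on their materials, replaying after random delays with a lightning particle burst.
; Other orphaned nodes would bob the puffs on phase-offset sine waves, reset flash colors and enable material wind.
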(event `self.ReceiveBeginPlay`)

(fn `Clouds`
  (params (`Lightning In` :type "Vector Structure") (NewParam1 :type "Vector Structure")))

(fn `UserConstructionScript`)