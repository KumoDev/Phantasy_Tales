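; BP_Ripple_Spline is a spline-based actor in the Sea content, apparently a base for ripple decals along a path.
; Its construction script loops over each segment between Spline points, adding a new spline component and decal component to the Decal's owner.
; Both are manually attached to the Spline with relative transforms; the script sets no per-segment placement or decal material.
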(fn `UserConstructionScript`
  (bind _spline (`self.Spline`))
  (bind _returnvalue (`ActorComponent.GetOwner` (`self.Decal`)))
  (for _ (range (+ (- (`SplineComponent.GetNumberOfSplinePoints` (`self.Spline`)) 2) 1))
    (bind _returnvalue_2 (`AddComponent|NODE_AddSplineComponent-2` :`self` _returnvalue :`bManualAttachment` true))
    (`SceneComponent.K2_AttachToComponent` _returnvalue_2 _spline "None" "KeepRelative" "KeepRelative" "KeepRelative" true)
    (bind _returnvalue_3 (`AddComponent|NODE_AddDecalComponent-3` :`self` _returnvalue :`bManualAttachment` true))
    (`SceneComponent.K2_AttachToComponent` _returnvalue_3 _spline "None" "KeepRelative" "KeepRelative" "KeepRelative" true)))