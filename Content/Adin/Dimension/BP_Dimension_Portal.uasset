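; Dimension portal actor that shifts the world into another dimension look when the player overlaps its box.
; BeginPlay caches MPC_Sky values and writes the box location to MPC_Dimension as the effect center.
; On overlap, a timeline grows the sphere, drives a temporary light and lerps both parameter collections.
; Each update sphere-traces for "Grid"-tagged components, swaps their material, then uses a delay before disabling collision and main-pass rendering.
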(event `self.Box.OnComponentBeginOverlap`
  (params (OverlappedComponent :type "PrimitiveComponent Object Reference") (OtherActor :type "Actor Object Reference") (OtherComp :type "PrimitiveComponent Object Reference") (OtherBodyIndex :type Integer) (bFromSweep :type Boolean) (SweepResult :type "HitResult Structure (by ref)"))
  (bind _pointlight (`self.PointLight`))
  (bind _returnvalue (`SceneComponent.K2_GetComponentLocation` (`self.Actor Referencer`)))
  (if (== OtherActor (`GameplayStatics.GetPlayerCharacter` 0))
    (bind (_direction _sphere_size_increase _everything_else _light_intensity _sphere) (`Timeline|Sphere Size` :!via `PlayFromStart`)
      (:`Update`
        (`SceneComponent.K2_SetRelativeTransform` (`self.Sphere`) (`KismetMathLibrary.MakeTransform` (0.0 0.0 0.0) (struct) (`KismetMathLibrary.Conv_DoubleToVector` (/ _sphere_size_increase 100.0))) true false)
        (`LightComponent.SetIntensity` _pointlight _light_intensity)
        (`KismetMaterialLibrary.SetScalarParameterValue` "/Game/Adin/Dimension/Mat/MPC_Dimension.MPC_Dimension" "Sphere Size" _sphere)
        (`KismetMaterialLibrary.SetScalarParameterValue` "/Game/Adin/Dimension/Mat/MPC_Sky.MPC_Sky" "Horizon Height" (`KismetMathLibrary.Lerp` (stale `self.ReceiveBeginPlay` _returnvalue) 243756793856.0 _everything_else))
        (`KismetMaterialLibrary.SetScalarParameterValue` "/Game/Adin/Dimension/Mat/MPC_Sky.MPC_Sky" "Horizon Falloff" (`KismetMathLibrary.Lerp` (stale `self.ReceiveBeginPlay` _returnvalue_2) 256.0 _everything_else))
        (`KismetMaterialLibrary.SetScalarParameterValue` "/Game/Adin/Dimension/Mat/MPC_Sky.MPC_Sky" "Zenith Height" (`KismetMathLibrary.Lerp` (stale `self.ReceiveBeginPlay` _returnvalue_3) -3579839.25 _everything_else))
        (`KismetMaterialLibrary.SetScalarParameterValue` "/Game/Adin/Dimension/Mat/MPC_Sky.MPC_Sky" "Zenith Falloff" (`KismetMathLibrary.Lerp` (stale `self.ReceiveBeginPlay` _returnvalue_4) 512.0 _everything_else))
        (`KismetMaterialLibrary.SetScalarParameterValue` "/Game/Adin/Dimension/Mat/MPC_Sky.MPC_Sky" "Brightness" (`KismetMathLibrary.Lerp` (stale `self.ReceiveBeginPlay` _returnvalue_5) 0.0 _everything_else))
        (`KismetMaterialLibrary.SetScalarParameterValue` "/Game/Adin/Dimension/Mat/MPC_Sky.MPC_Sky" "Sun Radius" (`KismetMathLibrary.Lerp` (stale `self.ReceiveBeginPlay` _returnvalue_6) 0.003 _everything_else))
        (`KismetMaterialLibrary.SetScalarParameterValue` "/Game/Adin/Dimension/Mat/MPC_Sky.MPC_Sky" "Sun Brightness" (`KismetMathLibrary.Lerp` (stale `self.ReceiveBeginPlay` _returnvalue_7) 0.0 _everything_else))
        (`KismetMaterialLibrary.SetScalarParameterValue` "/Game/Adin/Dimension/Mat/MPC_Sky.MPC_Sky" "Sun Glow Radius" (`KismetMathLibrary.Lerp` 0.0 0.003 _everything_else))
        (`KismetMaterialLibrary.SetScalarParameterValue` "/Game/Adin/Dimension/Mat/MPC_Sky.MPC_Sky" "Sun Glow Falloff" (`KismetMathLibrary.Lerp` (stale `self.ReceiveBeginPlay` _returnvalue_8) 0.0 _everything_else))
        (`KismetMaterialLibrary.SetScalarParameterValue` "/Game/Adin/Dimension/Mat/MPC_Sky.MPC_Sky" "Sun Glow Brightness" (`KismetMathLibrary.Lerp` (stale `self.ReceiveBeginPlay` _returnvalue_9) 0.0 _everything_else))
        (`KismetMaterialLibrary.SetVectorParameterValue` "/Game/Adin/Dimension/Mat/MPC_Sky.MPC_Sky" "Sun Color" (`KismetMathLibrary.LinearColorLerp` (stale `self.ReceiveBeginPlay` _returnvalue_10) (struct :`R` 1.0 :`G` 0.930111 :`B` 0.132868 :`A` 1.0) _everything_else))
        (`KismetMaterialLibrary.SetVectorParameterValue` "/Game/Adin/Dimension/Mat/MPC_Sky.MPC_Sky" "Sun Glow Color" (`KismetMathLibrary.LinearColorLerp` (stale `self.ReceiveBeginPlay` _returnvalue_11) (struct :`R` 1.0 :`G` 0.930111 :`B` 0.132868 :`A` 1.0) _everything_else))
        (`KismetMaterialLibrary.SetVectorParameterValue` "/Game/Adin/Dimension/Mat/MPC_Sky.MPC_Sky" "Horizon Color" (`KismetMathLibrary.LinearColorLerp` (stale `self.ReceiveBeginPlay` _returnvalue_12) (struct :`R` 0.090082 :`G` 0.184325 :`B` 0.348958 :`A` 1.0) _everything_else))
        (`KismetMaterialLibrary.SetVectorParameterValue` "/Game/Adin/Dimension/Mat/MPC_Sky.MPC_Sky" "Zenith Color" (`KismetMathLibrary.LinearColorLerp` (stale `self.ReceiveBeginPlay` _returnvalue_13) (struct :`R` 0.385417 :`G` 0.496783 :`B` 1.0 :`A` 1.0) _everything_else))
        (`KismetMaterialLibrary.SetVectorParameterValue` "/Game/Adin/Dimension/Mat/MPC_Sky.MPC_Sky" "Mid Color" (`KismetMathLibrary.LinearColorLerp` (stale `self.ReceiveBeginPlay` _returnvalue_14) (struct :`R` 0.285917 :`G` 0.389115 :`B` 0.871367 :`A` 1.0) _everything_else))
        (`KismetMaterialLibrary.SetScalarParameterValue` "/Game/Adin/Dimension/Mat/MPC_Dimension.MPC_Dimension" "2nd Shade" (`KismetMathLibrary.Lerp` 0.0 0.0 _everything_else))
        (`KismetMaterialLibrary.SetScalarParameterValue` "/Game/Adin/Dimension/Mat/MPC_Dimension.MPC_Dimension" "Metallic" (`KismetMathLibrary.Lerp` 0.0 0.01 _everything_else))
        (`KismetMaterialLibrary.SetScalarParameterValue` "/Game/Adin/Dimension/Mat/MPC_Dimension.MPC_Dimension" "Specularity" (`KismetMathLibrary.Lerp` 0.0 0.01 _everything_else))
        (`KismetMaterialLibrary.SetScalarParameterValue` "/Game/Adin/Dimension/Mat/MPC_Dimension.MPC_Dimension" "Roughness" (`KismetMathLibrary.Lerp` 0.0 0.8 _everything_else))
        (`KismetMaterialLibrary.SetScalarParameterValue` "/Game/Adin/Dimension/Mat/MPC_Dimension.MPC_Dimension" "Emissive" (`KismetMathLibrary.Lerp` 0.0 0.125 _everything_else))
        (bind _outhits (`KismetSystemLibrary.SphereTraceMulti` _returnvalue _returnvalue _sphere_size_increase "TraceTypeQuery1" false (`|MakeArray` (cast `/Game/Blueprints/Character/CH_MyCharacter` (`GameplayStatics.GetPlayerCharacter` 0) :!pure true) :!type "Actor Object Reference") "None" true (struct :`R` 1.0 :`A` 1.0) (struct :`G` 1.0 :`A` 1.0) 0.0))
        (for _array_element _outhits
          (if (`ActorComponent.ComponentHasTag` (`.HitComponent` (`GameplayStatics.BreakHitResult` _array_element)) "Grid")
            (bind _returnvalue_2 (`KismetArrayLibrary.Array_Add` (`self.Temp`)))
            (`KismetSystemLibrary.PrintString` (`KismetStringLibrary.Conv_IntToString` _returnvalue_2) true true (struct :`R` 0.017018 :`G` 0.340222 :`B` 1.0 :`A` 1.0))))
        (for _array_element_2 (`self.Temp`)
          (`PrimitiveComponent.SetMaterial` _array_element_2 0 "/Game/WorldAssets/Materials/Grid/Materials/MI_climbing_grid_dimension.MI_climbing_grid_dimension")
          (`KismetSystemLibrary.Delay` 3.0)
          (`self.SetActorEnableCollision` (`ActorComponent.GetOwner` _array_element_2) false)
          (`PrimitiveComponent.SetRenderInMainPass` _array_element_2 false))
        (`KismetSystemLibrary.PrintString` "mat changed"))
      (:`Finished`
        (`ActorComponent.K2_DestroyComponent` _pointlight)))))

(event `self.ReceiveBeginPlay`
  (bind (_origin _boxextent) (`self.GetActorBounds` (`self.Start Point`) false))
  (bind _output_get (set `self.Start Extent` _boxextent))
  (set `self.Start Extent` (- _output_get _origin))
  (bind _returnvalue (`KismetMaterialLibrary.GetScalarParameterValue` "/Game/Adin/Dimension/Mat/MPC_Sky.MPC_Sky" "Horizon Height"))
  (bind _returnvalue_2 (`KismetMaterialLibrary.GetScalarParameterValue` "/Game/Adin/Dimension/Mat/MPC_Sky.MPC_Sky" "Horizon Falloff"))
  (bind _returnvalue_3 (`KismetMaterialLibrary.GetScalarParameterValue` "/Game/Adin/Dimension/Mat/MPC_Sky.MPC_Sky" "Zenith Height"))
  (bind _returnvalue_4 (`KismetMaterialLibrary.GetScalarParameterValue` "/Game/Adin/Dimension/Mat/MPC_Sky.MPC_Sky" "Zenith Falloff"))
  (bind _returnvalue_5 (`KismetMaterialLibrary.GetScalarParameterValue` "/Game/Adin/Dimension/Mat/MPC_Sky.MPC_Sky" "Brightness"))
  (bind _returnvalue_6 (`KismetMaterialLibrary.GetScalarParameterValue` "/Game/Adin/Dimension/Mat/MPC_Sky.MPC_Sky" "Sun Radius"))
  (bind _returnvalue_7 (`KismetMaterialLibrary.GetScalarParameterValue` "/Game/Adin/Dimension/Mat/MPC_Sky.MPC_Sky" "Sun Brightness"))
  (bind _returnvalue_8 (`KismetMaterialLibrary.GetScalarParameterValue` "/Game/Adin/Dimension/Mat/MPC_Sky.MPC_Sky" "Sun Glow Radius"))
  (bind _returnvalue_9 (`KismetMaterialLibrary.GetScalarParameterValue` "/Game/Adin/Dimension/Mat/MPC_Sky.MPC_Sky" "Sun Glow Falloff"))
  (bind _returnvalue_10 (`KismetMaterialLibrary.GetVectorParameterValue` "/Game/Adin/Dimension/Mat/MPC_Sky.MPC_Sky" "Sun Color"))
  (bind _returnvalue_11 (`KismetMaterialLibrary.GetVectorParameterValue` "/Game/Adin/Dimension/Mat/MPC_Sky.MPC_Sky" "Sun Glow Color"))
  (bind _returnvalue_12 (`KismetMaterialLibrary.GetVectorParameterValue` "/Game/Adin/Dimension/Mat/MPC_Sky.MPC_Sky" "Horizon Color"))
  (bind _returnvalue_13 (`KismetMaterialLibrary.GetVectorParameterValue` "/Game/Adin/Dimension/Mat/MPC_Sky.MPC_Sky" "Zenith Color"))
  (bind _returnvalue_14 (`KismetMaterialLibrary.GetVectorParameterValue` "/Game/Adin/Dimension/Mat/MPC_Sky.MPC_Sky" "Mid Color"))
  (`KismetMaterialLibrary.SetVectorParameterValue` "/Game/Adin/Dimension/Mat/MPC_Dimension.MPC_Dimension" "Player Position" (`KismetMathLibrary.Conv_VectorToLinearColor` (`SceneComponent.K2_GetComponentLocation` (`self.Box`)))))

(fn `UserConstructionScript`)