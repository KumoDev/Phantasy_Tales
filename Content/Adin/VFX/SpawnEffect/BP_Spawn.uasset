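; BP_Spawn is a spawn visual effect actor that plays automatically on BeginPlay.
; It activates the PSpawn particle component, toggles a light, and writes a sphere location offset into the MPC_House material parameter collection.
; An EasyEase timeline then animates the collection's radius and particle radius alongside the light intensity, so materials reading MPC_House follow the effect, and deactivates the particles when finished.
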(event `self.ReceiveBeginPlay`
  (`ActorComponent.Activate` (`self.P_Spawn`) false)
  (`KismetMaterialLibrary.SetVectorParameterValue` "/Game/Adin/VFX/SpawnEffect/Materials/MPC_House.MPC_House" "Sphere Location Offset" (`KismetMathLibrary.Conv_VectorToLinearColor` (`self.Sphere Location Offset`)))
  (`ActorComponent.ToggleActive` (`self.Light`))
  (bind (_direction _radius _light _particle_radius) (`Timeline|Easy Ease` :`NewTime` 6.0 :!via `PlayFromStart`)
    (:`Update`
      (`KismetMaterialLibrary.SetScalarParameterValue` "/Game/Adin/VFX/SpawnEffect/Materials/MPC_House.MPC_House" "Radius" _radius)
      (`KismetMaterialLibrary.SetScalarParameterValue` "/Game/Adin/VFX/SpawnEffect/Materials/MPC_House.MPC_House" "Particle Radius" _particle_radius)
      (`LightComponent.SetIntensity` (`self.Light`) _light))
    (:`Finished`
      (`ActorComponent.Deactivate` (`self.P_Spawn`)))))

(fn `UserConstructionScript`)