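; Deer enemy AI that patrols random points around its spawn and runs to a distant random point when it sees a pawn.
; Tick drives patrol and walk speed, overriding the flee speed, with AttackCounter pausing movement after attacks.
; Hitbox overlaps target the player for attacks through a reused Bear AnimBP.
; Damage knocks it back, death scatters coins before destruction, and Selected handles the lock-on material.
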(event `self.ReceiveBeginPlay`
  (set `self.StartingLocation` (`self.K2_GetActorLocation`)) ; Store this so that they don't patrol too far away from their origin
  (if (!= (`self.Attack_counter`) 0)
    _))

(event `self.PawnSensing.OnSeePawn`
  (params (Pawn :type "Pawn Object Reference"))
  (bind _charactermovement (`self.CharacterMovement`))
  ;[1 1 1] RunAway
  (`|AIMoveTo` self (`NavigationSystem.K2_GetRandomLocationInNavigableRadius` (`self.K2_GetActorLocation`) 50000.0) null 40.0
    (:`then`
      (set `self.IsAttacking` true)
      (set `CharacterMovementComponent.MaxWalkSpeed` 1100.0 _charactermovement)
      (`KismetSystemLibrary.PrintString` (`KismetStringLibrary.Conv_DoubleToString` (`CharacterMovementComponent.MaxWalkSpeed` _charactermovement))))
    (:`OnSuccess`
      (set `self.IsAttacking` false))))

(event `self.ReceiveTick`
  (params (DeltaSeconds :type "Float (single-precision)"))
  (`|ExecutionSequence`
    (:`then_0`
      ;[1 1 1] Patrolling
      (if (== (`self.Attack_counter`) 1)
        (set `CharacterMovementComponent.MaxWalkSpeed` 0.0 (`self.CharacterMovement`))
        (else
          (set `CharacterMovementComponent.MaxWalkSpeed` 100.0 (`self.CharacterMovement`))
          (`/Engine/EditorBlueprintResources/StandardMacros.DoOnce` false :!label _label
            (:`Completed`
              (`|AIMoveTo` self (`NavigationSystem.K2_GetRandomLocationInNavigableRadius` (`self.StartingLocation`) (`self.PatrolRange`)) null 40.0
                (:`OnSuccess`
                  (goto _label :!via `Reset`))
                (:`OnFail`
                  (goto _label :!via `Reset`))))))))
    (:`then_1`
      (bind _asch_my_character (cast `/Game/Blueprints/Character/CH_MyCharacter` (`GameplayStatics.GetPlayerCharacter` 0)))
      (if (> (`/Game/Blueprints/Character/CH_MyCharacter.AttackCounter` _asch_my_character) 0)
        (set `self.Attack_counter` 0)))))

(event `self.Hitbox.OnComponentBeginOverlap`
  (params (OverlappedComponent :type "PrimitiveComponent Object Reference") (OtherActor :type "Actor Object Reference") (OtherComp :type "PrimitiveComponent Object Reference") (OtherBodyIndex :type Integer) (bFromSweep :type Boolean) (SweepResult :type "HitResult Structure (by ref)"))
  ;[1 1 1] DealingDamage
  (bind _asch_my_character (cast `/Game/Blueprints/Character/CH_MyCharacter` OtherActor))
  (set `self.TargetActor` _asch_my_character)
  (`self.AI_Attack`))

(event `self.ReceiveAnyDamage`
  (params (Damage :type "Float (single-precision)") (DamageType :type "DamageType Object Reference") (InstigatedBy :type "Controller Object Reference") (DamageCauser :type "Actor Object Reference"))
  (bind (_returnvalue_x _returnvalue_y _returnvalue_z) (`KismetMathLibrary.BreakVector` (`self.K2_GetActorLocation`)))
  (bind _currencyspread (`self.CurrencySpread`))
  ;[1 1 1] TakingDamage
  (bind _output_get (set `self.AI_CurrentHealth` (- (`self.AI_CurrentHealth`) Damage)))
  (`self.LaunchCharacter` (`KismetMathLibrary.MakeVector` (.x (* (`self.GetActorForwardVector`) -1000)) (.y (* (`self.GetActorForwardVector`) -1000)) (+ (.z (* (`self.GetActorForwardVector`) -1000)) 300.0)) true true)
  (if (<= _output_get 0.0)
    (`SkeletalMeshComponent.PlayAnimation` (`self.Mesh`) "/Game/Enemies/Slime_Enemy/Animations/Slime_Death_Anim.Slime_Death_Anim" false)
    (for _ (range (`self.Currency_MinDrop`) (+ (`self.Currency_MaxDrop`) 1))
      (`|SpawnActorFromClass` "/Game/Blueprints/Interactables/Currency/BPC_Coins.BPC_Coins_C" (`KismetMathLibrary.Conv_VectorToTransform` (`KismetMathLibrary.MakeVector` (+ _returnvalue_x (`KismetMathLibrary.RandomFloatInRange` 5.0 _currencyspread)) (+ _returnvalue_y (`KismetMathLibrary.RandomFloatInRange` 5.0 _currencyspread)) (+ _returnvalue_z (`KismetMathLibrary.RandomFloatInRange` 5.0 _currencyspread)))) "Undefined" "OverrideRootScale" null null))
    (`KismetSystemLibrary.Delay` 1.0)
    (`self.K2_DestroyActor`)))

(event `self.Hitbox.OnComponentEndOverlap`
  (params (OverlappedComponent :type "PrimitiveComponent Object Reference") (OtherActor :type "Actor Object Reference") (OtherComp :type "PrimitiveComponent Object Reference") (OtherBodyIndex :type Integer))
  ;[1 1 1] DealingDamage
  (bind _asch_my_character (cast `/Game/Blueprints/Character/CH_MyCharacter` OtherActor))
  (set `self.TargetActor` _asch_my_character))

(event `AI_Attack`
  ;[1 1 1] DealingDamage
  (if (!= (`self.Attack_counter`) 1)
    (bind _asbear_anim_bp (cast `/Game/WildLife/Bear/Bear_AnimBP` (`SkeletalMeshComponent.GetAnimInstance` (`self.Mesh`))))
    (set `/Game/WildLife/Bear/Bear_AnimBP.Attack` true _asbear_anim_bp)
    (`/Engine/EditorBlueprintResources/StandardMacros.IsValid` (`self.TargetActor`)
      (:`Is Valid`
        (`GameplayStatics.ApplyDamage` (`self.TargetActor`) (`self.DamageAmount`) null self)
        (`KismetSystemLibrary.Delay` 0.5)
        (cast `/Game/WildLife/Bear/Bear_AnimBP` (`SkeletalMeshComponent.GetAnimInstance` (`self.Mesh`)))
        (set `self.Attack_counter` 1))
      (:`Is Not Valid`
        (set `self.IsAttacking` false)))))

(fn `Selected`
  (params (InSelected :type Boolean))
  (if InSelected
    (`PrimitiveComponent.SetMaterial` (`self.Mesh`) 0 "/Game/ThirdPersonBP/Blueprints/LockOnMat.LockOnMat")
    (else
      (`PrimitiveComponent.SetMaterial` (`self.Mesh`) 0 null))))

(fn `UserConstructionScript`)