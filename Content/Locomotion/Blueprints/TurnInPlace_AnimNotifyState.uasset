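; Anim notify state that marks the turn-in-place window in animations played by the ALS locomotion anim blueprint.
; Begin, tick and end each cast the mesh's anim instance to ALS_AnimBP and call StartTurnInPlace, TurnInPlace and StopTurnInPlace respectively.
; The notify holds no turning logic itself, leaving that to the anim blueprint, and does nothing on other anim instances.
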(fn `Received_NotifyBegin`
  (params (MeshComp :type "SkeletalMeshComponent Object Reference") (Animation :type "AnimSequenceBase Object Reference") (TotalDuration :type "Float (double-precision)"))
  (returns (ReturnValue :type Boolean))
  (bind _asals_anim_bp (cast `/Game/Locomotion/Blueprints/ALS_AnimBP` (`SkeletalMeshComponent.GetAnimInstance` MeshComp))
    (:`then`
      (`/Game/Locomotion/Blueprints/ALS_AnimBP.StartTurnInPlace` _asals_anim_bp)
      (return true))
    (:`CastFailed`
      (return false))))

(fn `Received_NotifyEnd`
  (params (MeshComp :type "SkeletalMeshComponent Object Reference") (Animation :type "AnimSequenceBase Object Reference"))
  (returns (ReturnValue :type Boolean))
  (bind _asals_anim_bp (cast `/Game/Locomotion/Blueprints/ALS_AnimBP` (`SkeletalMeshComponent.GetAnimInstance` MeshComp))
    (:`then`
      (`/Game/Locomotion/Blueprints/ALS_AnimBP.StopTurnInPlace` _asals_anim_bp)
      (return false))
    (:`CastFailed`
      (return false))))

(fn `Received_NotifyTick`
  (params (MeshComp :type "SkeletalMeshComponent Object Reference") (Animation :type "AnimSequenceBase Object Reference") (FrameDeltaTime :type "Float (double-precision)"))
  (returns (ReturnValue :type Boolean))
  (bind _asals_anim_bp (cast `/Game/Locomotion/Blueprints/ALS_AnimBP` (`SkeletalMeshComponent.GetAnimInstance` MeshComp))
    (:`then`
      (`/Game/Locomotion/Blueprints/ALS_AnimBP.TurnInPlace` _asals_anim_bp)
      (return false))
    (:`CastFailed`
      (return false))))